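; BP_BushTile is a grid tile representing a bush that catches fire when hit.
; Its IHit handler runs the parent logic, then on the first hit sets IsOnFire and applies the fire effect, turning Stick4's material red.
; IApplyEffect, triggered on ignition, sends a one-damage hit message to the tile's Unit.
; BeginPlay fills a four-entry stick list, and ApplyHit and Hit forward to IHit with zero damage.
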(event `self.ReceiveBeginPlay`
  (`parent.ReceiveBeginPlay`)
  (`KismetArrayLibrary.Array_Add` (`self.SMSticksList`))
  (`KismetArrayLibrary.Array_Add` (`self.SMSticksList`))
  (`KismetArrayLibrary.Array_Add` (`self.SMSticksList`))
  (`KismetArrayLibrary.Array_Add` (`self.SMSticksList`)))

(event `ApplyHit`
  (`self.I_Hit` self null 0))

(event `Hit`
  (`self.I_Hit` null))

(event `/Game/GlobalBlueprints/Interface/I_Damageble.I_Hit`
  (params (fromWho :type "Actor Object Reference") (damage :type Integer))
  (`parent.I_Hit` fromWho damage)
  (if (not (`self.IsOnFire`))
    (`self.ApplyFireEffect`)
    (set `self.IsOnFire` true)))

(event `ApplyFireEffect`
  (`PrimitiveComponent.SetMaterial` (`self.Stick4`) 0 "/Game/Materials/MI_Red.MI_Red")
  (`/Game/Grid/Blueprints/Tile/Interface/I_Tile.I_ApplyEffect`))

(event `/Game/Grid/Blueprints/Tile/Interface/I_Tile.I_ApplyEffect`
  (message `/Game/GlobalBlueprints/Interface/I_Damageble.I_Hit` (`self.Unit`) self 1))

(fn `I_GetIdex`
  (returns (Index :type "IntPoint Structure"))
  (return))

(fn `UserConstructionScript`
  (`parent.UserConstructionScript`))