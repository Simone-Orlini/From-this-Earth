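; BP_Base_Tile is the base grid tile Blueprint, storing its index and the unit currently standing on it.
; It works through interface-style events and functions that set or return the index, track units entering and leaving, and forward hit damage to the occupant.
; A Border component, hidden at start, shows the tile state by swapping flat materials for hover, movement, attack, to-reach and combined highlights.
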(event `self.ReceiveBeginPlay`
  (`SceneComponent.SetHiddenInGame` (`self.Border`) true false))

(event `/Game/Grid/Blueprints/Tile/Interface/I_Tile.I_OnTileEnter`
  (params (Actor :type "Actor Object Reference"))
  (set `self.Unit` Actor))

(event `/Game/Grid/Blueprints/Tile/Interface/I_Tile.I_ShowBorder`
  (params (TileState :type "/Game/Grid/Blueprints/Tile/Utilites/E_TileState Enum" :default "NewEnumerator0"))
  (bind _border (`self.Border`))
  (if (`|EnumEquality` TileState "NewEnumerator0")
    (`SceneComponent.SetHiddenInGame` (`self.Border`) true false)
    (else
      (`SceneComponent.SetHiddenInGame` _border false false)
      (`PrimitiveComponent.SetMaterial` _border 0 (select `/Game/Grid/Blueprints/Tile/Utilites/E_TileState` TileState :`NewEnumerator0` "/Game/Grid/Material/MaterialForStaticMesh/TileInGame/MI_GridFlatSquare.MI_GridFlatSquare" :`NewEnumerator5` "/Game/Grid/Material/MaterialForStaticMesh/TileInGame/MI_GridFlatHovered.MI_GridFlatHovered" :`NewEnumerator1` "/Game/Grid/Material/MaterialForStaticMesh/TileInGame/MI_GridFlatMovement.MI_GridFlatMovement" :`NewEnumerator2` "/Game/Grid/Material/MaterialForStaticMesh/TileInGame/MI_GridFlatAttack.MI_GridFlatAttack" :`NewEnumerator6` "/Game/Grid/Material/MaterialForStaticMesh/TileInGame/MI_GridFlatToReach.MI_GridFlatToReach" :`NewEnumerator7` "/Game/Grid/Material/MaterialForStaticMesh/TileInGame/MI_GridFlatHoveredToReach.MI_GridFlatHoveredToReach" :`NewEnumerator8` "/Game/Grid/Material/MaterialForStaticMesh/TileInGame/MI_GridFlatMovementToReach.MI_GridFlatMovementToReach" :!type "MaterialInterface Object Reference")))))

(event `/Game/Grid/Blueprints/Interface/I_Gridable.I_SetIndex`
  (params (intdex :type "IntPoint Structure"))
  (set `self.Index` intdex))

(event `/Game/Grid/Blueprints/Tile/Interface/I_Tile.I_OnTileExit`
  (set `self.Unit` null))

(event `/Game/GlobalBlueprints/Interface/I_Damageble.I_Hit`
  (params (fromWho :type "Actor Object Reference") (damage :type Integer))
  (message `/Game/GlobalBlueprints/Interface/I_Damageble.I_Hit` (`self.Unit`) self damage))

(fn `I_GetIndex`
  (returns (index :type "IntPoint Structure"))
  (return (`self.Index`)))

(fn `I_GetUnit`
  (returns (Unit :type "Actor Object Reference"))
  (return (`self.Unit`)))

(fn `UserConstructionScript`)