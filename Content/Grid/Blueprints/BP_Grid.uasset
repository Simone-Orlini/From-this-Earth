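; Tile grid actor for grid-based movement and attacks, spawning grass, water and bush tile actors at BeginPlay.
; Construction draws a debug-line preview; baking ground-traces each cell, storing height-snapped tiles in BPCGridModifier and passing them to ACPathfinding and ACBFS.
; Spawned tiles are mapped by index for path queries, which are limited to highlighted tiles.
; Range highlights use BFS for hover and movement, straight cross lines for attack, shown through tile border interface messages.
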(event Custom|Bake_New
  (Default|Clear (Variables|Default|GetBPC_GridModifier))
  (CallFunction|BakeOld))

(event Custom|Show
  (bind (_keypin _valuepin) (Utilities|Map|ForEachLoop(Map) (Variables|/Game/Grid/Blueprints/Component/BPC_GridModifier.BPC_GridModifier_C|GetTiles (Variables|Default|GetBPC_GridModifier)))
    (:then
      (Default|ChangeTileTypewithIndex (Variables|Default|GetBPC_GridModifier) _keypin (.TileType (Utilities|Struct|BreakS_TileData _valuepin))))))

(event Custom|Bake_Old
  (bind _gridtilesize (Variables|Parameter|GetGridTileSize))
  (Variables|/Game/Grid/Blueprints/Component/AC_Pathfinding.AC_Pathfinding_C|SetZTileSize (Variables|Default|GetAC_Pathfinding) (.z _gridtilesize))
  (Variables|/Game/Grid/Blueprints/Component/AC_BFS.AC_BFS_C|SetZTileSize (Variables|Default|GetAC_BFS) (.z _gridtilesize))
  (Variables|Parameter|SetGridCenterLocation (Transformation|GetActorLocation))
  (Rendering|Debug|FlushPersistentDebugLines)
  (Generation|BakeGrid))

(event Custom|ResetTile
  (bind _valuepin (Utilities|Map|ForEachLoop(Map) (Variables|Default|GetTiles))
    (:then
      (Class|ITile|IShowBorder(Message) _valuepin "NewEnumerator0"))))

(event Custom|ResetOnlyTileInRange
  (for _array_element (Variables|Default|GetTileInRange)
    (switch Utilities|FlowControl|Switch|SwitchonE_TileState (Variables|/Game/Grid/Blueprints/Tile/BP_Base_Tile.BP_Base_Tile_C|GetTile%20State (.Value (Utilities|Map|Find (Variables|Default|GetTiles) _array_element)))
      (:NewEnumerator5
        (Class|ITile|IShowBorder(Message) (.Value (Utilities|Map|Find (Variables|Default|GetTiles) _array_element)) "NewEnumerator0" :!label _label))
      (:NewEnumerator1
        (goto _label))
      (:NewEnumerator2
        (goto _label))
      (:NewEnumerator7
        (Class|ITile|IShowBorder(Message) (.Value (Utilities|Map|Find (Variables|Default|GetTiles) _array_element)) "NewEnumerator6" :!label _label_2))
      (:NewEnumerator8
        (goto _label_2)))))

(event EventBeginPlay
  (Generation|SpawnGrid))

(fn ConstructionScript
  (Variables|/Game/Grid/Blueprints/Component/BPC_GridModifier.BPC_GridModifier_C|SetGridTileSize (Variables|Default|GetBPC_GridModifier) (Variables|Parameter|GetGridTileSize))
  (Variables|/Game/Grid/Blueprints/Component/BPC_GridModifier.BPC_GridModifier_C|SetGridSize (Variables|Default|GetBPC_GridModifier) (Variables|Parameter|GetGridSize))
  (Variables|Parameter|SetGridCenterLocation (Transformation|GetActorLocation))
  (Generation|DrawGrid))

(fn DrawGrid
  (bind _gridsize (Variables|Parameter|GetGridSize))
  (bind _gridsize_2 (Variables|Parameter|GetGridSize))
  (bind (_center _bottonleft) (Generation|CalculateCenterandBottonLeft))
  (Variables|Parameter|SetGridCenterLocation _center)
  (Variables|Parameter|SetGridBottomLeftLocation _bottonleft)
  (LocalVariables|SetOffset (* (Variables|Parameter|GetGridTileSize) "0.500000,0.500000,-0.050000"))
  (Rendering|Debug|FlushPersistentDebugLines)
  (if (and (Variables|Debug|GetUseEnvarioment) (not (Variables|Debug|GetDrawFullGrid)))
    (Variables|Debug|SetDrawFullGrid true)
    (elif (and (not (Variables|Debug|GetDrawFullGrid)) (Variables|Debug|GetUseEnvarioment))
      (Variables|Debug|SetUseEnvarioment false)))
  (if (Variables|Debug|GetDrawFullGrid)
    (for _index (range 0 (- (* (.x _gridsize) (.y _gridsize)) 1))
      (LocalVariables|SetX (Math|Integer|%(Integer) _index (.x _gridsize_2)))
      (LocalVariables|SetY (/ _index (.x _gridsize_2)))
      (LocalVariables|SetTileLocation (+ (Variables|Parameter|GetGridBottomLeftLocation) (* (Variables|Parameter|GetGridTileSize) (Math|Vector|MakeVector (Math|Conversions|ToFloat(Integer) (LocalVariables|GetX)) (Math|Conversions|ToFloat(Integer) (LocalVariables|GetY)) 0.0))))
      (if (Variables|Debug|GetUseEnvarioment)
        (bind (_hitsomething _outlocation) (Generation|TraceforGround (LocalVariables|GetTileLocation)))
        (if _hitsomething
          (LocalVariables|SetTileLocation (- _outlocation (LocalVariables|GetOffset)))
          ;[0.15 0.15 0.15 0.5] Horizontal Line
          (Rendering|Debug|DrawDebugLine (LocalVariables|GetTileLocation) (+ (LocalVariables|GetTileLocation) (Math|Vector|MakeVector (.x (Variables|Parameter|GetGridTileSize)) 0.0 0.0)) (Variables|Debug|GetLine%20Color) (LocalVariables|GetLineDuration) (Variables|Debug|GetLine%20Thickness))
          ;[0.15 0.15 0.15 0.5] Vertical Line
          (Rendering|Debug|DrawDebugLine (LocalVariables|GetTileLocation) (+ (LocalVariables|GetTileLocation) (Math|Vector|MakeVector 0.0 (.y (Variables|Parameter|GetGridTileSize)) 0.0)) (Variables|Debug|GetLine%20Color) (LocalVariables|GetLineDuration) (Variables|Debug|GetLine%20Thickness)))
        (else
          (LocalVariables|SetTileLocation (- (LocalVariables|GetTileLocation) (LocalVariables|GetOffset)))
          ;[0.15 0.15 0.15 0.5] Horizontal Line
          (Rendering|Debug|DrawDebugLine (LocalVariables|GetTileLocation) (+ (LocalVariables|GetTileLocation) (Math|Vector|MakeVector (.x (Variables|Parameter|GetGridTileSize)) 0.0 0.0)) (Variables|Debug|GetLine%20Color) (LocalVariables|GetLineDuration) (Variables|Debug|GetLine%20Thickness))
          ;[0.15 0.15 0.15 0.5] Vertical Line
          (Rendering|Debug|DrawDebugLine (LocalVariables|GetTileLocation) (+ (LocalVariables|GetTileLocation) (Math|Vector|MakeVector 0.0 (.y (Variables|Parameter|GetGridTileSize)) 0.0)) (Variables|Debug|GetLine%20Color) (LocalVariables|GetLineDuration) (Variables|Debug|GetLine%20Thickness)))))
    (else
      ;[0.15 0.15 0.15 0.5] Draw only the square with the grid size
      (Utilities|FlowControl|Sequence
        (:then_0
          (LocalVariables|SetTileLocation (- (Variables|Parameter|GetGridBottomLeftLocation) (LocalVariables|GetOffset)))
          (Rendering|Debug|DrawDebugLine (LocalVariables|GetTileLocation) (+ (LocalVariables|GetTileLocation) (Math|Vector|MakeVector (* (.x (Variables|Parameter|GetGridTileSize)) (.x (Variables|Parameter|GetGridSize))) 0.0 0.0)) (Variables|Debug|GetLine%20Color) (LocalVariables|GetLineDuration) (Variables|Debug|GetLine%20Thickness)))
        (:then_1
          (Rendering|Debug|DrawDebugLine (LocalVariables|GetTileLocation) (+ (LocalVariables|GetTileLocation) (Math|Vector|MakeVector 0.0 (* (.y (Variables|Parameter|GetGridTileSize)) (.y (Variables|Parameter|GetGridSize))) 0.0)) (Variables|Debug|GetLine%20Color) (Variables|Debug|GetLine%20Thickness) (Variables|Debug|GetLine%20Thickness)))
        (:then_2
          (Rendering|Debug|DrawDebugLine (+ (LocalVariables|GetTileLocation) (Math|Vector|MakeVector (* (.x (Variables|Parameter|GetGridTileSize)) (.x (Variables|Parameter|GetGridSize))) 0.0 0.0)) (+ (+ (LocalVariables|GetTileLocation) (Math|Vector|MakeVector (* (.x (Variables|Parameter|GetGridTileSize)) (.x (Variables|Parameter|GetGridSize))) 0.0 0.0)) (Math|Vector|MakeVector 0.0 (* (.y (Variables|Parameter|GetGridTileSize)) (.y (Variables|Parameter|GetGridSize))) 0.0)) (Variables|Debug|GetLine%20Color) (LocalVariables|GetLineDuration) (Variables|Debug|GetLine%20Thickness)))
        (:then_3
          (Rendering|Debug|DrawDebugLine (+ (LocalVariables|GetTileLocation) (Math|Vector|MakeVector 0.0 (* (.y (Variables|Parameter|GetGridTileSize)) (.y (Variables|Parameter|GetGridSize))) 0.0)) (+ (+ (LocalVariables|GetTileLocation) (Math|Vector|MakeVector 0.0 (* (.y (Variables|Parameter|GetGridTileSize)) (.y (Variables|Parameter|GetGridSize))) 0.0)) (Math|Vector|MakeVector (* (.x (Variables|Parameter|GetGridTileSize)) (.x (Variables|Parameter|GetGridSize))) 0.0 0.0)) (Variables|Debug|GetLine%20Color) (LocalVariables|GetLineDuration) (Variables|Debug|GetLine%20Thickness)))))))

(fn CalculateCenterandBottonLeft
  (bind _gridsize (Variables|Parameter|GetGridSize))
  (LocalVariables|SetC (CallFunction|SnapVectortoVector (Variables|Parameter|GetGridCenterLocation) (Variables|Parameter|GetGridTileSize)))
  (return (LocalVariables|GetC) (- (LocalVariables|GetC) (* (* (- (Math|Conversions|ToVector2D(Vector) (Variables|Parameter|GetGridSize)) (Math|Vector2D|MakeVector2D (Math|Conversions|ToFloat(Integer) (Math|Integer|SelectInt 0 1 (CallFunction|IsIntEven (.x _gridsize)))) (Math|Conversions|ToFloat(Integer) (Math|Integer|SelectInt 0 1 (CallFunction|IsIntEven (.y _gridsize)))))) 0.5) (Math|Conversions|ToVector2D(Vector) (Variables|Parameter|GetGridTileSize))))))

(fn TraceforGround
  (params (Location :type Vector))
  ;[0.15 0.15 0.15 0.5] Cambiare con un line trace
  (bind (_outhit _returnvalue) (Collision|LineTraceByChannel (+ Location "0.000000,0.000000,1000.000000") (- Location "0.000000,0.000000,100.000000") "TraceTypeQuery3" false 0 "None" true "(R=1.000000,G=0.000000,B=0.000000,A=1.000000)" "(R=0.000000,G=1.000000,B=0.000000,A=1.000000)" 0.5))
  (if _returnvalue
    (return true (Math|Vector|MakeVector (.x Location) (.y Location) (+ (Math|Float|SnapToGrid(Float) (.Z (Math|Vector|BreakVector (.Location (Collision|BreakHitResult _outhit)))) (* (.z (Variables|Parameter|GetGridTileSize)) 0.5)) 1.0)))
    (else
      (return false Location))))

(fn GetTileIndexfromWorldLocation
  (params (Location :type Vector))
  (bind _output_get (LocalVariables|SetLocationOnGrid (- Location (Variables|Parameter|GetGridBottomLeftLocation))))
  (LocalVariables|SetSnappedLocationOnGrid (Math|Conversions|ToVector2D(Vector) (CallFunction|SnapVectortoVector _output_get (Variables|Parameter|GetGridTileSize))))
  (return (Class|KismetMathLibrary|ToIntPoint(Vector2D) (/ (LocalVariables|GetSnappedLocationOnGrid) (Math|Conversions|ToVector2D(Vector) (Variables|Parameter|GetGridTileSize))))))

(fn BakeGrid
  (bind _gridsize (Variables|Parameter|GetGridSize))
  (bind _gridsize_2 (Variables|Parameter|GetGridSize))
  (bind _bpc_gridmodifier (Variables|Default|GetBPC_GridModifier))
  (bind _tilestocreate (Variables|/Game/Grid/Blueprints/Component/BPC_GridModifier.BPC_GridModifier_C|GetTilesToCreate _bpc_gridmodifier))
  (Utilities|Map|Clear (Variables|/Game/Grid/Blueprints/Component/BPC_GridModifier.BPC_GridModifier_C|GetTilesToCreate (Variables|Default|GetBPC_GridModifier)))
  (bind (_center _bottonleft) (Generation|CalculateCenterandBottonLeft))
  (Variables|Parameter|SetGridCenterLocation _center)
  (Variables|Parameter|SetGridBottomLeftLocation _bottonleft)
  (for _index (range 0 (- (* (.x _gridsize) (.y _gridsize)) 1))
    (LocalVariables|SetX (Math|Integer|%(Integer) _index (.x _gridsize_2)))
    (LocalVariables|SetY (/ _index (.x _gridsize_2)))
    (LocalVariables|SetTileTransform (Math|Transform|MakeTransform (+ (Variables|Parameter|GetGridBottomLeftLocation) (* (Variables|Parameter|GetGridTileSize) (Math|Vector|MakeVector (Math|Conversions|ToFloat(Integer) (LocalVariables|GetX)) (Math|Conversions|ToFloat(Integer) (LocalVariables|GetY)) 0.0))) "0, 0, 0" "1.000000,1.000000,1.000000"))
    (LocalVariables|SetIndex (Utilities|Struct|MakeIntPoint (LocalVariables|GetX) (LocalVariables|GetY)))
    (bind (_hitsomething _outlocation) (Generation|TraceforGround (.location (LocalVariables|GetTileTransform))))
    (if _hitsomething
      (Default|GenerateTile (Variables|Default|GetBPC_GridModifier) (Utilities|Struct|MakeS_TileData (LocalVariables|GetIndex) (Math|Transform|MakeTransform _outlocation (.rotation (LocalVariables|GetTileTransform)) (.scale (LocalVariables|GetTileTransform))) "NewEnumerator0"))
      (Variables|/Game/Grid/Blueprints/Component/AC_Pathfinding.AC_Pathfinding_C|SetTiles (Variables|Default|GetAC_Pathfinding) _tilestocreate)
      (Variables|/Game/Grid/Blueprints/Component/AC_BFS.AC_BFS_C|SetTiles (Variables|Default|GetAC_BFS) _tilestocreate)
      (else
        (Default|RemoveTile (Variables|Default|GetBPC_GridModifier) (LocalVariables|GetIndex))))))

(fn SpawnGrid
  (Rendering|Debug|FlushPersistentDebugLines)
  (bind _valuepin (Utilities|Map|ForEachLoop(Map) (Variables|/Game/Grid/Blueprints/Component/BPC_GridModifier.BPC_GridModifier_C|GetTilesToCreate (Variables|Default|GetBPC_GridModifier)))
    (:then
      (Generation|CreateGridTile _valuepin))))

(fn CreateGridTile
  (params (TileData :type S%20Tile%20Data%20Structure))
  (switch Utilities|FlowControl|Switch|SwitchonE_TileType (.tiletype TileData)
    (:NewEnumerator0
      (Development|PrintString "No Type for the Tile" true true "(R=1.000000,G=0.026075,B=0.000000,A=1.000000)" 1e+01))
    (:NewEnumerator1
      (LocalVariables|SetTileToSpawn "/Game/Grid/Blueprints/Tile/BP_GrassTile.BP_GrassTile_C")
      (bind _returnvalue (Game|SpawnActorfromClass (LocalVariables|GetTileToSpawn) (.transform TileData) "Undefined" "MultiplyWithRoot" 0 0 :!label _label))
      (bind _asbp_base_tile (Utilities|Casting|CastToBP_Base_Tile _returnvalue))
      (Variables|/Game/Grid/Blueprints/Tile/BP_Base_Tile.BP_Base_Tile_C|SetIndex _asbp_base_tile (.index TileData))
      (Utilities|Map|Add (Variables|Default|GetTiles) (.index TileData) _asbp_base_tile))
    (:NewEnumerator2
      (LocalVariables|SetTileToSpawn "/Game/Grid/Blueprints/Tile/BP_WaterTile.BP_WaterTile_C")
      (goto _label))
    (:NewEnumerator3
      (LocalVariables|SetTileToSpawn "/Game/Grid/Blueprints/Tile/BP_BushTile.BP_BushTile_C")
      (goto _label))))

(fn InstantiateTiles)

(fn IsinRange
  (params (Tile :type Int%20Point%20Structure))
  (return (Utilities|Array|ContainsItem (Variables|Default|GetTileInRange) Tile)))

(fn FindPath
  (params (StartNode :type Int%20Point%20Structure) (TargetNode :type Int%20Point%20Structure))
  (if (Utilities|Array|ContainsItem (Variables|Default|GetTileInRange) TargetNode)
    (bind _path (Default|FindPath (Variables|Default|GetAC_Pathfinding) StartNode TargetNode))
    (for _array_element _path
      (if (.ReturnValue (Utilities|Map|Find (Variables|Default|GetTiles) _array_element))
        (Utilities|Array|Add (LocalVariables|GetTilesLocation) (Transformation|GetActorLocation (.Value (Utilities|Map|Find (Variables|Default|GetTiles) _array_element))))))
    (return (LocalVariables|GetTilesLocation))
    (else
      (return (LocalVariables|GetTilesLocation)))))

(fn FindTile
  (params (Index :type Int%20Point%20Structure))
  (return (.Value (Utilities|Map|Find (Variables|Default|GetTiles) Index))))

(fn ShowTiles
  (params (TileState :type E_TileState%20Enum :default "NewEnumerator0") (StartNode :type Int%20Point%20Structure) (Range :type Integer))
  (CallFunction|ResetOnlyTileinRange)
  (switch Utilities|FlowControl|Switch|SwitchonE_TileState TileState
    (:NewEnumerator5
      (bind _tiles (Default|GetTilesinRange (Variables|Default|GetAC_BFS) StartNode Range :!label _label))
      (Utilities|Array|RemoveItem _tiles StartNode)
      (CallFunction|UpdateTilesBorder _tiles TileState))
    (:NewEnumerator1
      (goto _label))
    (:NewEnumerator2
      (while (<= (LocalVariables|GetI) Range)
        (Utilities|Array|AppendArray (LocalVariables|GetArrayToReturn) (Utilities|Array|MakeArray (+ StartNode (Utilities|Struct|MakeIntPoint (LocalVariables|GetI) 0)) (+ StartNode (Utilities|Struct|MakeIntPoint 0 (LocalVariables|GetI))) (+ StartNode (Utilities|Struct|MakeIntPoint (* (LocalVariables|GetI) -1) 0)) (+ StartNode (Utilities|Struct|MakeIntPoint 0 (* (LocalVariables|GetI) -1)))))
        (Math|Integer|IncrementInt (LocalVariables|GetI)))
      (CallFunction|UpdateTilesBorder (LocalVariables|GetArrayToReturn) "NewEnumerator2"))))

(fn GetRandomTileIndex
  (return (.Key (Utilities|Map|GetKeyValueByIndex (Variables|Default|GetTiles) (Math|Random|RandomInteger (Utilities|Map|Length (Variables|Default|GetTiles)))))))

(fn ShowTiletoReach
  (params (Index :type Int%20Point%20Structure))
  (CallFunction|HideTiletoReach (Variables|Default|GetTileToReach))
  (Variables|Default|SetTileToReach Index)
  (Class|ITile|IShowBorder(Message) (.Value (Utilities|Map|Find (Variables|Default|GetTiles) Index)) "NewEnumerator6"))

(fn HideTiletoReach
  (params (Index :type Int%20Point%20Structure))
  (Class|ITile|IShowBorder(Message) (.Value (Utilities|Map|Find (Variables|Default|GetTiles) Index)) "NewEnumerator0")
  (Variables|Default|SetTileToReach (Utilities|Struct|MakeIntPoint -1 -1)))

(fn UpdateTilesBorder
  (params (Tiles :type Array%20of%20Int%20Point%20Structures) (TileState :type E_TileState%20Enum :default "NewEnumerator0"))
  (bind _tiletoreach (Variables|Default|GetTileToReach))
  (bind _value (Utilities|Map|Find (Variables|Default|GetTiles) _tiletoreach))
  (bind _output_get (Variables|Default|SetTileInRange Tiles))
  (for _array_element _output_get
    (Class|ITile|IShowBorder(Message) (.Value (Utilities|Map|Find (Variables|Default|GetTiles) _array_element)) TileState))
  (if (Utilities|Array|ContainsItem (Variables|Default|GetTileInRange) (Variables|Default|GetTileToReach))
    (switch Utilities|FlowControl|Switch|SwitchonE_TileState TileState
      (:NewEnumerator5
        (Class|ITile|IShowBorder(Message) _value "NewEnumerator7"))
      (:NewEnumerator1
        (Class|ITile|IShowBorder(Message) _value "NewEnumerator8")))))

(fn ShowTilebyIndex
  (params (Index :type Int%20Point%20Structure) (TileState :type E_TileState%20Enum :default "NewEnumerator0"))
  (Variables|Default|SetTileToReach Index)
  (Class|ITile|IShowBorder(Message) (.Value (Utilities|Map|Find (Variables|Default|GetTiles) Index)) TileState))