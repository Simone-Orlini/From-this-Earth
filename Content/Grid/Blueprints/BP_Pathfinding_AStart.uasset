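; A* pathfinder that returns the tile path between two grid points, excluding the start node.
; AStar fills CameFrom and CostSoFar using uniform step cost plus straight-line distance, and FindPath walks CameFrom back and reverses it.
; Neighbors are the four adjacent tiles in GridRef's modifier whose height differs by at most one tile height.
; The frontier is a map scanned linearly for lowest priority; queued nodes keep their first priority.
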(fn `AddUnique`
  (params (Key :type "IntPoint Structure (by ref)") (Value :type "Float (double-precision) (by ref)"))
  (bind _frontier (`self.Frontier`))
  (if (not (`.ReturnValue` (`BlueprintMapLibrary.Map_Find` _frontier Key)))
    (`BlueprintMapLibrary.Map_Add` _frontier Key Value)))

(fn `AStar`
  (params (startNode :type "IntPoint Structure (by ref)") (endNode :type "IntPoint Structure"))
  (locals (defaultCost :type Integer :default 1) (currentNode :type "IntPoint Structure") (newCost :type Integer) (Neighbor :type "IntPoint Structure") (priority :type "Float (double-precision)"))
  (`BlueprintMapLibrary.Map_Add` (`self.CameFrom`) startNode startNode)
  (`BlueprintMapLibrary.Map_Add` (`self.CostSoFar`) startNode (`local.defaultCost`))
  (`self.AddUnique` (`local.startNode`) (`self.Heuristic` (`local.startNode`) (`local.endNode`)))
  (while (not (`BlueprintMapLibrary.Map_IsEmpty` (`self.Frontier`)))
    (bind _output_get (set `local.currentNode` (`self.GetBestNode`)))
    (if (`/Game/Grid/Blueprints/Utilities/BPF_Utilities.IsIntPointsEqual` _output_get (`local.endNode`))
      (return)
      (else
        (for _array_element (`self.GetValidNeightbor` (`local.currentNode`))
          (set `local.Neighbor` _array_element)
          (set `local.newCost` (+ (`BlueprintMapLibrary.Map_Find` (`self.CostSoFar`) (`local.currentNode`)) (`local.defaultCost`)))
          (if (or (not (`BlueprintMapLibrary.Map_Contains` (`self.CostSoFar`) (`local.Neighbor`))) (> (`BlueprintMapLibrary.Map_Find` (`self.CostSoFar`) (`local.Neighbor`)) (`local.newCost`)))
            (`BlueprintMapLibrary.Map_Add` (`self.CameFrom`) (`local.Neighbor`) (`local.currentNode`))
            (`BlueprintMapLibrary.Map_Add` (`self.CostSoFar`) (`local.Neighbor`) (`local.newCost`))
            (set `local.priority` (+ (`local.newCost`) (`self.Heuristic` (`local.Neighbor`) (`local.endNode`))))
            (`self.AddUnique` (`local.Neighbor`) (`local.priority`))))))))

(fn `FindPath`
  (params (startNode :type "IntPoint Structure") (targetNode :type "IntPoint Structure"))
  (returns (Path :type "Array of IntPoint Structure"))
  (locals (pathToReturn :type "Array of IntPoint Structure") (currentNode :type "IntPoint Structure"))
  (bind _pathtoreturn (`local.pathToReturn`))
  (`BlueprintMapLibrary.Map_Clear` (`self.CameFrom`))
  (`BlueprintMapLibrary.Map_Clear` (`self.CostSoFar`))
  (`BlueprintMapLibrary.Map_Clear` (`self.Frontier`))
  (if (or (`/Game/Grid/Blueprints/Utilities/BPF_Utilities.IsOutsideGrid` (`local.startNode`)) (`/Game/Grid/Blueprints/Utilities/BPF_Utilities.IsOutsideGrid` (`local.targetNode`)))
    (return)
    (else
      (`self.AStar` (`local.startNode`) (`local.targetNode`))
      (if (not (`BlueprintMapLibrary.Map_Contains` (`self.CameFrom`) (`local.targetNode`)))
        (return)
        (else
          (bind _output_get (set `local.currentNode` (`local.targetNode`)))
          (while (!= _output_get (`BlueprintMapLibrary.Map_Find` (`self.CameFrom`) (`local.currentNode`)))
            (`KismetArrayLibrary.Array_Add` (`local.pathToReturn`) (`local.currentNode`))
            (set `local.currentNode` (`BlueprintMapLibrary.Map_Find` (`self.CameFrom`) (`local.currentNode`))))
          (`KismetArrayLibrary.Array_Reverse` _pathtoreturn)
          (return _pathtoreturn))))))

(fn `GetBestNode`
  (returns (retNode :type "IntPoint Structure"))
  (locals (node :type "IntPoint Structure") (lowestPriority :type "Float (double-precision)" :default 2.0) (flaotMaxValue :type "Float (double-precision)" :default 4294967295.0) (currentPriority :type "Float (double-precision)"))
  (set `local.lowestPriority` (`local.flaotMaxValue`))
  (bind _keys (`BlueprintMapLibrary.Map_Keys` (`self.Frontier`)))
  (for _array_element _keys
    (bind _output_get (set `local.currentPriority` (`BlueprintMapLibrary.Map_Find` (`self.Frontier`) _array_element)))
    (if (< _output_get (`local.lowestPriority`))
      (set `local.lowestPriority` (`local.currentPriority`))
      (set `local.node` _array_element)))
  (`BlueprintMapLibrary.Map_Remove` (`self.Frontier`) (`local.node`))
  (return (`local.node`)))

(fn `GetValidNeightbor`
  (params (Node :type "IntPoint Structure"))
  (returns (Neighbors :type "Array of IntPoint Structure"))
  (locals (neighbors_Arr :type "Array of IntPoint Structure"))
  (bind (_gridtilesize_x _gridtilesize_y _gridtilesize_z) (`KismetMathLibrary.BreakVector` (`/Game/Grid/Blueprints/BP_Grid.GridTileSize` (`self.Grid_Ref`))))
  (for _array_element (`|MakeArray` (+ (`local.Node`) (make `IntPoint` 1)) (+ (`local.Node`) (make `IntPoint` 0 1)) (+ (`local.Node`) (make `IntPoint` -1)) (+ (`local.Node`) (make `IntPoint` 0 -1)))
    (bind (_value _returnvalue) (`BlueprintMapLibrary.Map_Find` (`/Game/Grid/Blueprints/BP_GridModifier.Tiles` (`/Game/Grid/Blueprints/BP_Grid.GridModifier_ref` (`self.Grid_Ref`))) _array_element))
    (if _returnvalue
      (if (<= (`KismetMathLibrary.Abs` (- (.z (.location (`.Transform_6_5A67382A40DF1E1E6E48B4B8CB8455CF` (break `/Game/Grid/Blueprints/Tile/Utilites/S_TileData` _value)))) (.z (.location (`.Transform_6_5A67382A40DF1E1E6E48B4B8CB8455CF` (break `/Game/Grid/Blueprints/Tile/Utilites/S_TileData` (`BlueprintMapLibrary.Map_Find` (`/Game/Grid/Blueprints/BP_GridModifier.Tiles` (`/Game/Grid/Blueprints/BP_Grid.GridModifier_ref` (`self.Grid_Ref`))) (`local.Node`)))))))) _gridtilesize_z)
        (`KismetArrayLibrary.Array_Add` (`local.neighbors_Arr`) (break `/Game/Grid/Blueprints/Tile/Utilites/S_TileData` _value)))))
  (return (`local.neighbors_Arr`)))

(fn `Heuristic`
  (params (start :type "IntPoint Structure") (end :type "IntPoint Structure"))
  (returns (manhattanDistance :type "Float (double-precision)"))
  (bind (_returnvalue_x _returnvalue_y) (break `IntPoint` (- start end)))
  (return (`KismetMathLibrary.Abs` (`KismetMathLibrary.Sqrt` (`KismetMathLibrary.Conv_IntToDouble` (+ (* _returnvalue_x _returnvalue_x) (* _returnvalue_y _returnvalue_y)))))))

(fn `UserConstructionScript`)