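; BPC_GridModifier is a component that stores the grid's tiles and their terrain types: None, Grass, Water or Bush.
; A map keyed by tile index holds each transform and type, with functions to generate, retype, look up, remove or clear entries.
; Regenerating an existing tile keeps its type, while new tiles get the default.
; Generating or retyping a tile draws a timed debug plane colored by type.
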(fn `ChangeTileColor`
  (params (Location :type "Vector Structure") (TileType :type "/Game/Grid/Blueprints/Tile/Utilites/E_TileType Enum" :default "NewEnumerator0"))
  (`KismetSystemLibrary.DrawDebugPlane` (`KismetMathLibrary.MakePlaneFromPointAndNormal` Location (0.0 0.0 -1.0)) Location (- (.x (* (`self.GridTileSize`) (0.5 0.5 0.0))) 5.0) (select `/Game/Grid/Blueprints/Tile/Utilites/E_TileType` (`local.TileType`) :`NewEnumerator1` (struct :`R` 0.75969 :`G` 1.0 :`A` 1.0) :`NewEnumerator2` (struct :`G` 0.902542 :`B` 1.0 :`A` 1.0) :`NewEnumerator3` (struct :`R` 0.006762 :`G` 0.119792 :`B` 0.003704 :`A` 1.0) :!type "LinearColor Structure") (`self.Duration`)))

(fn `ChangeTileType`
  (params (TileType :type "/Game/Grid/Blueprints/Tile/Utilites/E_TileType Enum" :default "NewEnumerator0") (I :type Integer))
  (locals (index :type "IntPoint Structure") (Tile :type "/Game/Grid/Blueprints/Tile/Utilites/S_TileData Structure"))
  (bind _gridsize_x (break `IntVector2` (`self.GridSize`)))
  (`self.ChangeTileTypeWithIndex` (make `IntPoint` (mod I _gridsize_x) (/ I _gridsize_x)) TileType))

(fn `ChangeTileTypeWithIndex`
  (params (Index :type "IntPoint Structure (by ref)") (`Tile Type` :type "/Game/Grid/Blueprints/Tile/Utilites/E_TileType Enum" :default "NewEnumerator0"))
  (bind _value (`BlueprintMapLibrary.Map_Find` (`self.Tiles`) Index))
  (`BlueprintMapLibrary.Map_Add` (`self.Tiles`) Index (make `/Game/Grid/Blueprints/Tile/Utilites/S_TileData` (break `/Game/Grid/Blueprints/Tile/Utilites/S_TileData` _value) (`.Transform_6_5A67382A40DF1E1E6E48B4B8CB8455CF` (break `/Game/Grid/Blueprints/Tile/Utilites/S_TileData` _value)) (`local.Tile Type`)))
  (`self.ChangeTileColor` (.location (`.Transform_6_5A67382A40DF1E1E6E48B4B8CB8455CF` (break `/Game/Grid/Blueprints/Tile/Utilites/S_TileData` _value))) (`local.Tile Type`)))

(fn `Clear`
  (`BlueprintMapLibrary.Map_Clear` (`self.Tiles`)))

(fn `GenerateTile`
  (params (TileData :type "/Game/Grid/Blueprints/Tile/Utilites/S_TileData Structure"))
  (bind (_tiledata_index _tiledata_transform) (break `/Game/Grid/Blueprints/Tile/Utilites/S_TileData` (`local.TileData`)))
  (bind _tiledata_index_2 (break `/Game/Grid/Blueprints/Tile/Utilites/S_TileData` (`local.TileData`)))
  (bind (_value _returnvalue) (`BlueprintMapLibrary.Map_Find` (`self.Tiles`) (`.Index_7_4E91E8A442C0FDADDCC3F7B41AA0E665` (break `/Game/Grid/Blueprints/Tile/Utilites/S_TileData` TileData))))
  (bind _value_2 (`BlueprintMapLibrary.Map_Find` (`self.Tiles`) _tiledata_index_2))
  (`BlueprintMapLibrary.Map_Add` (`self.Tiles`) _tiledata_index (make `/Game/Grid/Blueprints/Tile/Utilites/S_TileData` _tiledata_index _tiledata_transform (select `bool` _returnvalue :`false` (`self.DefaultTileType`) :`true` (`.TileType_17_9DD958A34384116033DE17A85D142752` (break `/Game/Grid/Blueprints/Tile/Utilites/S_TileData` _value)))))
  (`self.ChangeTileColor` (.location (`.Transform_6_5A67382A40DF1E1E6E48B4B8CB8455CF` (break `/Game/Grid/Blueprints/Tile/Utilites/S_TileData` _value_2))) (`.TileType_17_9DD958A34384116033DE17A85D142752` (break `/Game/Grid/Blueprints/Tile/Utilites/S_TileData` _value_2))))

(fn `GetTile`
  (params (Index :type "IntPoint Structure (by ref)"))
  (returns (TileData :type "/Game/Grid/Blueprints/Tile/Utilites/S_TileData Structure") (IsFound :type Boolean))
  (bind (_value _returnvalue) (`BlueprintMapLibrary.Map_Find` (`self.Tiles`) Index))
  (return _value _returnvalue))

(fn `RemoveTile`
  (params (Index :type "IntPoint Structure"))
  (`BlueprintMapLibrary.Map_Remove` (`self.Tiles`) Index))