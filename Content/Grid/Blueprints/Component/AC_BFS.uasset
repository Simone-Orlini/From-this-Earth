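; Grid pathfinding component that returns the tiles reachable within a given range of a start node, using breadth-first search.
; GetTilesInRange resets the search state, rejects off-grid starts, then runs BFS with a queue-style Frontier and uniform step cost tracked in CostSoFar.
; GetValidNeighbor supplies four-directional neighbors that exist in Tiles, are not yet collected, and differ in height by at most half ZTileSize.
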(fn `BFS`
  (params (StartNode :type "IntPoint Structure") (Range :type Integer))
  (locals (defaultCost :type Integer :default 1) (neighbor :type "IntPoint Structure") (currentNode :type "IntPoint Structure") (newCost :type Integer) (neighbors :type "Array of IntPoint Structure"))
  (bind _frontier (`self.Frontier`))
  (bind _frontier_2 (`self.Frontier`))
  (`BlueprintMapLibrary.Map_Add` (`self.CostSoFar`) StartNode)
  (`KismetArrayLibrary.Array_Add` _frontier StartNode)
  (while (not (`KismetArrayLibrary.Array_IsEmpty` _frontier))
    (set `local.currentNode` (`|GetArrayItem` _frontier_2))
    (`KismetArrayLibrary.Array_Remove` _frontier_2)
    (bind _output_get (set `local.neighbors` (`self.GetValidNeighbor` (`local.currentNode`))))
    (for _array_element _output_get
      (set `local.neighbor` _array_element)
      (bind _output_get_2 (set `local.newCost` (+ (`BlueprintMapLibrary.Map_Find` (`self.CostSoFar`) (`local.currentNode`)) (`local.defaultCost`))))
      (if (not (> _output_get_2 (`local.Range`)))
        (`KismetArrayLibrary.Array_Add` (`self.TilesToReturn`) (`local.neighbor`))
        (`BlueprintMapLibrary.Map_Add` (`self.CostSoFar`) (`local.neighbor`) (`local.newCost`))
        (`KismetArrayLibrary.Array_Add` (`self.Frontier`) (`local.neighbor`))))))

(fn `GetTilesInRange`
  (params (StartNode :type "IntPoint Structure") (Range :type Integer) (ZTileSize :type "Float (double-precision)" :default 50.0))
  (returns (Tiles :type "Array of IntPoint Structure"))
  (set `self.ZTileSize` ZTileSize)
  (`KismetArrayLibrary.Array_Clear` (`self.Frontier`))
  (`BlueprintMapLibrary.Map_Clear` (`self.CostSoFar`))
  (`KismetArrayLibrary.Array_Clear` (`self.TilesToReturn`))
  (if (`/Game/Grid/Blueprints/Utilities/BPF_Utilities.IsOutsideGrid` (`local.StartNode`))
    (return)
    (else
      (`self.BFS` (`local.StartNode`) (`local.Range`))
      (return (`self.TilesToReturn`)))))

(fn `GetValidNeighbor`
  (params (Node :type "IntPoint Structure"))
  (returns (Neighbors :type "Array of IntPoint Structure"))
  (locals (neighbors_Arr :type "Array of IntPoint Structure"))
  (for _array_element (`|MakeArray` (`/Game/Grid/Blueprints/Utilities/BPF_Utilities.GetNodeFromPoint` (`local.Node`) 1) (`/Game/Grid/Blueprints/Utilities/BPF_Utilities.GetNodeFromPoint` (`local.Node`) 0 1) (`/Game/Grid/Blueprints/Utilities/BPF_Utilities.GetNodeFromPoint` (`local.Node`) -1) (`/Game/Grid/Blueprints/Utilities/BPF_Utilities.GetNodeFromPoint` (`local.Node`) 0 -1))
    (bind (_value _returnvalue) (`BlueprintMapLibrary.Map_Find` (`self.Tiles`) _array_element))
    (if _returnvalue
      (if (<= (`KismetMathLibrary.Abs` (- (.z (.location (`.Transform` (break `GridTileData` _value)))) (.z (.location (`.Transform` (break `GridTileData` (`BlueprintMapLibrary.Map_Find` (`self.Tiles`) (`local.Node`)))))))) (* (`self.ZTileSize`) 0.5))
        (if (not (`KismetArrayLibrary.Array_Contains` (`self.TilesToReturn`) _array_element))
          (`KismetArrayLibrary.Array_Add` (`local.neighbors_Arr`) _array_element)))))
  (return (`local.neighbors_Arr`)))