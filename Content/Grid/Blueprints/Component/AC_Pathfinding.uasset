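; Grid pathfinding component that runs A* between two tile coordinates and returns the steps, excluding the start.
; FindPath rejects off-grid endpoints, runs AStar, then walks the CameFrom map back from the target and reverses it.
; AStar uses uniform step cost plus straight-line distance, linearly scanning a Frontier map whose queued priorities are never updated.
; Neighbors are four-directional, filtered to height differences within half a tile's Z size.
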(fn `AddUnique`
  (params (Key :type "IntPoint Structure (by ref)") (Value :type "Float (double-precision) (by ref)"))
  (bind _frontier (`self.Frontier`))
  (if (not (`.ReturnValue` (`BlueprintMapLibrary.Map_Find` _frontier Key)))
    (`BlueprintMapLibrary.Map_Add` _frontier Key Value)))

(fn `AStar`
  (params (startNode :type "IntPoint Structure (by ref)") (endNode :type "IntPoint Structure"))
  (locals (defaultCost :type Integer :default 1) (currentNode :type "IntPoint Structure") (Neighbor :type "IntPoint Structure") (newCost :type Integer) (priority :type "Float (double-precision)") (Neighbors :type "Array of IntPoint Structure"))
  (`BlueprintMapLibrary.Map_Add` (`self.CameFrom`) startNode startNode)
  ; If each tiles have them own cost, change it
  (`BlueprintMapLibrary.Map_Add` (`self.CostSoFar`) startNode (`local.defaultCost`))
  (`self.AddUnique` (`local.startNode`) (`self.Heuristic` (`local.startNode`) (`local.endNode`)))
  (while (not (`BlueprintMapLibrary.Map_IsEmpty` (`self.Frontier`)))
    (bind _output_get (set `local.currentNode` (`self.GetBestNode`)))
    (if (`/Game/Grid/Blueprints/Utilities/BPF_Utilities.IsIntPointsEqual` _output_get (`local.endNode`))
      (return)
      (else
        (bind _output_get_2 (set `local.Neighbors` (`self.GetValidNeightbor` (`local.currentNode`))))
        (for _array_element _output_get_2
          (set `local.Neighbor` _array_element)
          (set `local.newCost` (+ (`BlueprintMapLibrary.Map_Find` (`self.CostSoFar`) (`local.currentNode`)) (`local.defaultCost`)))
          (if (or (not (`BlueprintMapLibrary.Map_Contains` (`self.CostSoFar`) (`local.Neighbor`))) (> (`BlueprintMapLibrary.Map_Find` (`self.CostSoFar`) (`local.Neighbor`)) (`local.newCost`)))
            (`BlueprintMapLibrary.Map_Add` (`self.CameFrom`) (`local.Neighbor`) (`local.currentNode`))
            (`BlueprintMapLibrary.Map_Add` (`self.CostSoFar`) (`local.Neighbor`) (`local.newCost`))
            (set `local.priority` (+ (`local.newCost`) (`self.Heuristic` (`local.Neighbor`) (`local.endNode`))))
            (`self.AddUnique` (`local.Neighbor`) (`local.priority`))))))))

(fn `FindPath`
  (params (StartNode :type "IntPoint Structure") (TargetNode :type "IntPoint Structure"))
  (returns (Path :type "Array of IntPoint Structure"))
  (locals (currentNode :type "IntPoint Structure") (pathToReturn :type "Array of IntPoint Structure"))
  (bind _pathtoreturn (`local.pathToReturn`))
  (`BlueprintMapLibrary.Map_Clear` (`self.CameFrom`))
  (`BlueprintMapLibrary.Map_Clear` (`self.CostSoFar`))
  (`BlueprintMapLibrary.Map_Clear` (`self.Frontier`))
  (if (or (`/Game/Grid/Blueprints/Utilities/BPF_Utilities.IsOutsideGrid` (`local.StartNode`)) (`/Game/Grid/Blueprints/Utilities/BPF_Utilities.IsOutsideGrid` (`local.TargetNode`)))
    (return)
    (else
      (`self.AStar` (`local.startNode`) (`local.targetNode`))
      (if (not (`BlueprintMapLibrary.Map_Contains` (`self.CameFrom`) (`local.targetNode`)))
        (return)
        (else
          (bind _output_get (set `local.currentNode` (`local.targetNode`)))
          (while (!= _output_get (`BlueprintMapLibrary.Map_Find` (`self.CameFrom`) (`local.currentNode`)))
            (`KismetArrayLibrary.Array_Add` (`local.pathToReturn`) (`local.currentNode`))
            (set `local.currentNode` (`BlueprintMapLibrary.Map_Find` (`self.CameFrom`) (`local.currentNode`))))
          (`KismetArrayLibrary.Array_Reverse` _pathtoreturn)
          (return _pathtoreturn))))))

(fn `GetBestNode`
  (returns (retNode :type "IntPoint Structure"))
  (locals (flaotMaxValue :type "Float (double-precision)" :default 4294967295.0) (lowestPriority :type "Float (double-precision)") (currentPriority :type "Float (double-precision)") (node :type "IntPoint Structure"))
  (set `local.lowestPriority` (`local.flaotMaxValue`))
  (bind _keys (`BlueprintMapLibrary.Map_Keys` (`self.Frontier`)))
  (for _array_element _keys
    (bind _output_get (set `local.currentPriority` (`BlueprintMapLibrary.Map_Find` (`self.Frontier`) _array_element)))
    (if (< _output_get (`local.lowestPriority`))
      (set `local.lowestPriority` (`local.currentPriority`))
      (set `local.node` _array_element)))
  (`BlueprintMapLibrary.Map_Remove` (`self.Frontier`) (`local.node`))
  (return (`local.node`)))

(fn `GetValidNeightbor`
  (params (Node :type "IntPoint Structure"))
  (returns (Neighbors :type "Array of IntPoint Structure"))
  (locals (neighbors_Arr :type "Array of IntPoint Structure"))
  (for _array_element (`|MakeArray` (+ (`local.Node`) (make `IntPoint` 1)) (+ (`local.Node`) (make `IntPoint` 0 1)) (+ (`local.Node`) (make `IntPoint` -1)) (+ (`local.Node`) (make `IntPoint` 0 -1)))
    (if true
      (bind _value (`BlueprintMapLibrary.Map_Find` (`self.Tiles`) _array_element))
      (if (<= (`KismetMathLibrary.Abs` (- (.z (.location (`.Transform_6_5A67382A40DF1E1E6E48B4B8CB8455CF` (break `/Game/Grid/Blueprints/Tile/Utilites/S_TileData` _value)))) (.z (.location (`.Transform_6_5A67382A40DF1E1E6E48B4B8CB8455CF` (break `/Game/Grid/Blueprints/Tile/Utilites/S_TileData` (`BlueprintMapLibrary.Map_Find` (`self.Tiles`) (`local.Node`)))))))) (* (`self.ZTileSize`) 0.5))
        (`KismetArrayLibrary.Array_Add` (`local.neighbors_Arr`) (break `/Game/Grid/Blueprints/Tile/Utilites/S_TileData` _value)))))
  (return (`local.neighbors_Arr`)))

(fn `Heuristic`
  (params (start :type "IntPoint Structure") (end :type "IntPoint Structure"))
  (returns (manhattanDistance :type "Float (double-precision)"))
  (bind (_returnvalue_x _returnvalue_y) (break `IntPoint` (- start end)))
  (return (`KismetMathLibrary.Abs` (`KismetMathLibrary.Sqrt` (`KismetMathLibrary.Conv_IntToDouble` (+ (* _returnvalue_x _returnvalue_x) (* _returnvalue_y _returnvalue_y)))))))