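; Grid modifier Blueprint that holds a map of tile overrides (index, transform, tile type) and draws them as mesh instances.
; Its construction script initializes the child-actor BP_GridMeshInstance once when GridRef is valid, printing an error otherwise, then re-adds every stored tile.
; Generate records a tile with DefaultTileType and adds its instance, while Clear empties both the map and the instances.
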(fn `Clear`
  (`BlueprintMapLibrary.Map_Clear` (`self.Tiles`))
  (`/Game/Grid/Blueprints/Utilities/BP_GridMeshInstance.ClearInstances` (`self.GridMeshInst`)))

(fn `Generate`
  (params (TileData :type "/Game/Grid/Blueprints/Tile/Utilites/S_TileData Structure"))
  (bind (_tiledata_index _tiledata_transform) (break `/Game/Grid/Blueprints/Tile/Utilites/S_TileData` (`local.TileData`)))
  (bind (_tiledata_index_2 _tiledata_transform_2) (break `/Game/Grid/Blueprints/Tile/Utilites/S_TileData` (`local.TileData`)))
  (set `self.GridMeshInst` (cast `/Game/Grid/Blueprints/Utilities/BP_GridMeshInstance` (`ChildActorComponent.ChildActor` (`self.ChildActor_GridMeshInst`)) :!pure true))
  (`BlueprintMapLibrary.Map_Add` (`self.Tiles`) _tiledata_index_2 (make `/Game/Grid/Blueprints/Tile/Utilites/S_TileData` _tiledata_index_2 _tiledata_transform_2 (`self.DefaultTileType`)))
  (`/Game/Grid/Blueprints/Utilities/BP_GridMeshInstance.AddOrUpdateInstance` (`self.GridMeshInst`) _tiledata_index _tiledata_transform (`self.DefaultTileType`)))

(fn `UserConstructionScript`
  (if (`self.HasItiliazed`)
    (set `self.GridMeshInst` (cast `/Game/Grid/Blueprints/Utilities/BP_GridMeshInstance` (`ChildActorComponent.ChildActor` (`self.ChildActor_GridMeshInst`)) :!pure true) :!label _label)
    (bind (_keypin _valuepin) (`|MapForEach` (`self.Tiles`))
      (:`then`
        (`/Game/Grid/Blueprints/Utilities/BP_GridMeshInstance.AddOrUpdateInstance` (`self.GridMeshInst`) (break `/Game/Grid/Blueprints/Tile/Utilites/S_TileData` _valuepin) (`.Transform_6_5A67382A40DF1E1E6E48B4B8CB8455CF` (break `/Game/Grid/Blueprints/Tile/Utilites/S_TileData` _valuepin)) (`.TileType_17_9DD958A34384116033DE17A85D142752` (break `/Game/Grid/Blueprints/Tile/Utilites/S_TileData` _valuepin)))))
    (else
      (`|ExecutionSequence`
        (:`then_0`
          (`self.Grid_ref`
            (:`then`
              (`/Game/Grid/Blueprints/Utilities/BP_GridMeshInstance.InitializeGridMeshInst` (`self.GridMeshInst`) "/Game/Grid/StaticMesh/SM_GridSquare_Plane.SM_GridSquare_Plane" "/Game/Grid/Material/MaterialForStaticMesh/TileInGame/M_GridFlat.M_GridFlat" (struct :`A` 1.0) "QueryOnly")
              (set `self.HasItiliazed` true))
            (:`else`
              (`KismetSystemLibrary.PrintString` "Grid ref doesn't setted in Grid Modifier" true true (struct :`R` 1.0 :`G` 9.5e-05 :`B` 0.024274 :`A` 1.0) 10.0))))
        (:`then_1`
          (goto _label))))))