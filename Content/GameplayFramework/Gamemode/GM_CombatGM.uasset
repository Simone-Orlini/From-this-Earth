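; Combat GameMode for a turn-based grid tactics game, coordinating BP_Grid, a turn system and an AI manager.
; Tile clicks select friendly units, then move them along grid paths or attack through their AC_Combat component, while Tick previews movement range under the cursor.
; Units register through interface calls, turn changes start enemy AI, and interface getters expose units, paths and ranges.
; A random mission tile relocates when reached, revealing a button after several hits.
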(event `self.ReceiveBeginPlay`
  (bind _returnvalue (`GameplayStatics.GetActorOfClass` "/Game/Grid/Blueprints/BP_Grid.BP_Grid_C"))
  (bind _output_get (set `self.GridRef` _returnvalue))
  (bind _output_get_2 (set `self.MissionTile` (`/Game/Grid/Blueprints/BP_Grid.GetRandomTileIndex` _output_get)))
  (`/Game/Grid/Blueprints/BP_Grid.ShowTileToReach` (`self.GridRef`) _output_get_2)
  (add `/Game/GameplayFramework/Gamemode/BPC_TurnSystem.TeamWon` (`self.BPC_TurnSystem`) (`|CreateDelegate` :!event `Event OnWin`))
  (add `/Game/GameplayFramework/Gamemode/BPC_TurnSystem.ChangeTurn` (`self.BPC_TurnSystem`) (`|CreateDelegate` :!event `Event OnChangeTurn`))
  (add `/Game/AI/AC_AIManager.OnLogicEnd` (`self.AC_AIManager`) (`|CreateDelegate` :!event `Event OnLogicEnd`)))

(event `/Game/GameplayFramework/Gamemode/Interfaces/BPI_GamemodeComunication.I_OnTileClick`
  (params (HitPosition :type "Vector Structure") (HitActor :type "Actor Object Reference"))
  (bind _gridref (`self.GridRef`))
  (bind _selectedunit (`self.SelectedUnit`))
  ; Tile pressed
  (`/Game/GameplayFramework/Gamemode/BPC_TurnSystem.PlayerTurn` (`self.BPC_TurnSystem`)
    (:`then`
      (bind _index (`/Game/Grid/Blueprints/BP_Grid.GetTileIndexFromWorldLocation` _gridref HitPosition))
      (bind (_value _returnvalue) (`BlueprintMapLibrary.Map_Find` (`/Game/Grid/Blueprints/BP_Grid.Tiles` _gridref) _index))
      (if _returnvalue
        (if (not (`self.IsAttacking`))
          (bind _unitfound (`self.SelectUnit` _value _index))
          (if (and (not _unitfound) (`KismetSystemLibrary.IsValid` _selectedunit))
            (bind _index_2 (message `/Game/Grid/Blueprints/Interface/I_Gridable.I_GetTileIndex` _selectedunit))
            (`self.IsAttacking`
              (:`then`
                (`self.UnitAttack` (`self.SelectedUnit`) _index_2)
                (set `self.SelectedUnit` null))
              (:`else`
                (`self.MoveUnit` _selectedunit _index_2 _index)
                (set `self.SelectedUnit` null))))
          (elif (not (== (`self.GetUnitFromTileIndex` _index) _selectedunit))
            (`self.UnitAttack` _selectedunit _index)))))
    (:`else`)))

(event `/Game/GameplayFramework/Gamemode/Interfaces/BPI_GamemodeComunication.I_OnTileReached`
  (params (TileIndex :type "IntPoint Structure"))
  (bind _maskthreshold (`self.MaskThreshold`))
  (bind _gridref (`self.GridRef`))
  ; Tile reached
  (if (<= (`self.MaskThreshold`) 3)
    (if (`KismetMathLibrary.Equal_IntPointIntPoint` TileIndex (`self.MissionTile`))
      (`/Game/UI/Mask/BP_FuctionLibrary.ShowPoint` _maskthreshold)
      (bind _result (`/Engine/EditorBlueprintResources/StandardMacros.IncrementInt` _maskthreshold)
        (:`  `
          (if (>= _result 3)
            (`/Game/UI/Mask/BP_FuctionLibrary.ShowButton`)
            (`/Game/Grid/Blueprints/BP_Grid.HideTileToReach` _gridref (`self.MissionTile`))
            (set `self.MissionTile` (make `IntPoint` -1 -1))
            (else
              (bind _output_get (set `self.MissionTile` (`/Game/Grid/Blueprints/BP_Grid.GetRandomTileIndex` (`self.GridRef`))))
              (`/Game/Grid/Blueprints/BP_Grid.ShowTileToReach` _gridref _output_get))))))))

(event `/Game/GameplayFramework/Gamemode/Interfaces/BPI_GamemodeComunication.I_SwitchTo`
  (params (State :type "/Game/Grid/Blueprints/Tile/Utilites/E_TileState Enum" :default "NewEnumerator0"))
  (bind _selectedunit (`self.SelectedUnit`))
  ; Switch to attack
  (`self.SelectedUnit`
    (:`then`
      (switch `/Game/Grid/Blueprints/Tile/Utilites/E_TileState` State
        (:`NewEnumerator1`
          (bind _canmove (message `/Game/Units/Blueprints/Interface/I_Unit.I_CanMove` _selectedunit))
          (if _canmove
            (set `self.IsAttacking` false)
            (bind _index (message `/Game/Grid/Blueprints/Interface/I_Gridable.I_GetTileIndex` _selectedunit))
            (bind _unitdata (message `/Game/Units/Blueprints/Interface/I_Unit.I_GetData` _selectedunit))
            (`/Game/Grid/Blueprints/BP_Grid.ShowMovementTiles` (`self.GridRef`) "NewEnumerator1" _index (`/Game/Units/Blueprints/Datas/BP_UnitData.MovementRange` _unitdata) 50.0)))
        (:`NewEnumerator2`
          (bind _canattack (message `/Game/Units/Blueprints/Interface/I_Unit.I_CanAttack` _selectedunit))
          (if _canattack
            (set `self.IsAttacking` true)
            (bind _index_2 (message `/Game/Grid/Blueprints/Interface/I_Gridable.I_GetTileIndex` _selectedunit))
            (bind _unitdata_2 (message `/Game/Units/Blueprints/Interface/I_Unit.I_GetData` _selectedunit))
            (`/Game/Grid/Blueprints/BP_Grid.ShowAttackTiles` (`self.GridRef`) _index_2 (`/Game/Units/Blueprints/Datas/BP_UnitData.WeaponData` _unitdata_2))))))
    (:`else`)))

(event `/Game/GameplayFramework/Gamemode/Interfaces/BPI_GamemodeComunication.I_SubscribeUnitToGameMode`
  (params (Unit :type "Actor Object Reference"))
  (`self.AddUnit` Unit))

(event `/Game/GameplayFramework/Gamemode/Interfaces/BPI_GamemodeComunication.I_UnsubscribeUnitFromGameMode`
  (params (Unit :type "Actor Object Reference"))
  (`self.RemoveUnit` Unit))

(event `self.ReceiveTick`
  (params (DeltaSeconds :type "Float (single-precision)"))
  (`self.CheckUnitHover`))

(event `/Game/GameplayFramework/Gamemode/Interfaces/BPI_GamemodeComunication.I_Attack`
  (params (Unit :type "Actor Object Reference") (TileIndexToAttack :type "IntPoint Structure"))
  (`/Game/GlobalBlueprints/Componets/AC_Combat.Attack` (`self.GetComponentByClass` Unit "/Game/GlobalBlueprints/Componets/AC_Combat.AC_Combat_C") (`/Game/Grid/Blueprints/BP_Grid.FindTile` (`self.GridRef`) TileIndexToAttack)))

(event `/Game/GameplayFramework/Gamemode/Interfaces/BPI_GamemodeComunication.I_EndTurn`
  (`/Game/GameplayFramework/Gamemode/BPC_TurnSystem.EndCurrentTurn` (`self.BPC_TurnSystem`)))

(event `Event OnChangeTurn`
  (params (IsPlayerTurn :type Boolean))
  (bind _bpc_turnsystem (`self.BPC_TurnSystem`))
  (if (not IsPlayerTurn)
    (`/Game/AI/AC_AIManager.StartAITurn` (`self.AC_AIManager`) (`/Game/GameplayFramework/Gamemode/BPC_TurnSystem.FriendlyUnits` _bpc_turnsystem) (`/Game/GameplayFramework/Gamemode/BPC_TurnSystem.EnemyUnits` _bpc_turnsystem))))

(event `/Game/GameplayFramework/Gamemode/Interfaces/BPI_GamemodeComunication.I_EndUnitTurn`
  (`/Game/GameplayFramework/Gamemode/BPC_TurnSystem.StartEnemyAI` (`self.BPC_TurnSystem`)))

(event `Event OnWin`
  (params (IsPlayer :type Boolean))
  (if IsPlayer
    (`KismetSystemLibrary.PrintString` "Player has won")
    (else
      (`KismetSystemLibrary.PrintString` "Enemy has won"))))

(event `Event OnLogicEnd`
  (`/Game/GameplayFramework/Gamemode/BPC_TurnSystem.StartEnemyAI` (`self.BPC_TurnSystem`)))

(fn `AddUnit`
  (params (Unit :type "Actor Object Reference"))
  (bind _unitdata (message `/Game/Units/Blueprints/Interface/I_Unit.I_GetData` Unit))
  (`/Game/Units/Blueprints/Datas/BP_UnitData.Friendly` _unitdata
    (:`then`
      (`KismetArrayLibrary.Array_AddUnique` (`/Game/GameplayFramework/Gamemode/BPC_TurnSystem.FriendlyUnits` (`self.BPC_TurnSystem`)) (`local.Unit`)))
    (:`else`
      (`KismetArrayLibrary.Array_AddUnique` (`/Game/GameplayFramework/Gamemode/BPC_TurnSystem.EnemyUnits` (`self.BPC_TurnSystem`)) (`local.Unit`)))))

(fn `CheckUnitHover`
  (locals (UnderCursorUnit :type "Actor Object Reference") (PrevUnderCursorTile :type "/Game/Grid/Blueprints/Tile/BP_Base_Tile Object Reference"))
  (bind _location (`self.GetCursorLocationOnGrid` 0))
  (bind _index (`/Game/Grid/Blueprints/BP_Grid.GetTileIndexFromWorldLocation` (`self.GridRef`) _location))
  (set `local.PrevUnderCursorTile` (`self.UnderCursorTile`))
  (bind (_value _returnvalue) (`BlueprintMapLibrary.Map_Find` (`/Game/Grid/Blueprints/BP_Grid.Tiles` (`self.GridRef`)) _index))
  (set `self.UnderCursorTile` _value)
  (if _returnvalue
    (if (!= (`self.UnderCursorTile`) (`local.PrevUnderCursorTile`))
      (bind _unit (`/Game/Grid/Blueprints/Tile/BP_Base_Tile.I_GetUnit` (`self.UnderCursorTile`)))
      (`/Engine/EditorBlueprintResources/StandardMacros.IsValid` _unit
        (:`Is Valid`
          (bind _output_get (set `local.UnderCursorUnit` _unit))
          (`self.SelectedUnit`
            (:`then`)
            (:`else`
              (bind _unitdata (message `/Game/Units/Blueprints/Interface/I_Unit.I_GetData` _output_get))
              (if (`KismetSystemLibrary.DoesImplementInterface` _output_get "/Game/Units/Blueprints/Interface/I_Unit.I_Unit_C")
                (`/Game/Grid/Blueprints/BP_Grid.ShowMovementTiles` (`self.GridRef`) "NewEnumerator5" (`/Game/Grid/Blueprints/Tile/BP_Base_Tile.Index` (`self.UnderCursorTile`)) (`/Game/Units/Blueprints/Datas/BP_UnitData.MovementRange` _unitdata) 50.0)
                (else
                  (`/Game/Grid/Blueprints/BP_Grid.ResetOnlyTileInRange` (`self.GridRef`) :!label _label))))))
        (:`Is Not Valid`
          (`local.PrevUnderCursorTile` :!label _label_2
            (:`then`
              (`self.SelectedUnit`
                (:`then`)
                (:`else`
                  (set `local.UnderCursorUnit` null)
                  (goto _label))))
            (:`else`)))))
    (else
      (goto _label_2))))

(fn `GetAllUnits`
  (returns (Units :type "Array of Actor Object Reference"))
  (locals (AllUnits :type "Array of Actor Object Reference"))
  (bind _bpc_turnsystem (`self.BPC_TurnSystem`))
  (bind _output_get (set `local.AllUnits` (`/Game/GameplayFramework/Gamemode/BPC_TurnSystem.FriendlyUnits` _bpc_turnsystem)))
  (`KismetArrayLibrary.Array_Append` _output_get (`/Game/GameplayFramework/Gamemode/BPC_TurnSystem.EnemyUnits` _bpc_turnsystem))
  (return (`local.AllUnits`)))

(fn `GetCursorLocationOnGrid`
  (params (PlayerIndex :type Integer))
  (returns (Location :type "Vector Structure"))
  (bind (_hitresult _returnvalue) (`PlayerController.GetHitResultUnderCursorByChannel` (`GameplayStatics.GetPlayerController` 0) "TraceTypeQuery4" false))
  (if _returnvalue
    (return (`.Location` (`GameplayStatics.BreakHitResult` _hitresult)))
    (else
      (return (-99999.0 -99999.0 -99999.0)))))

(fn `GetUnitFromTile`
  (params (TileRef :type "/Game/Grid/Blueprints/Tile/BP_Base_Tile Object Reference"))
  (returns (Unit :type "Actor Object Reference") (UnitFound :type Boolean))
  (bind _unit (message `/Game/Grid/Blueprints/Tile/Interface/I_Tile.I_GetUnit` TileRef))
  (return _unit (`KismetSystemLibrary.IsValid` _unit)))

(fn `GetUnitFromTileIndex`
  (params (TileIndex :type "IntPoint Structure"))
  (returns (Unit :type "Actor Object Reference") (UnitFound :type Boolean))
  (locals (Found :type Boolean))
  (bind (_value _returnvalue) (`BlueprintMapLibrary.Map_Find` (`/Game/Grid/Blueprints/BP_Grid.Tiles` (`self.GridRef`)) TileIndex))
  (bind _output_get (set `local.Found` _returnvalue))
  (if _output_get
    ; Setto e basta perché potrei arrivare anche dall'altra esecuzione
    (bind (_unit _unitfound) (`self.GetUnitFromTile` _value))
    (set `local.Found` _unitfound))
  (return _unit (`local.Found`)))

(fn `I_CheckAttack`
  (params (Unit :type "Actor Object Reference") (Tile :type "IntPoint Structure") (TileToCheck :type "IntPoint Structure"))
  (returns (CanAttack :type Boolean))
  (return (`/Game/Grid/Blueprints/BP_Grid.CheckAttack` (`self.GridRef`) Tile TileToCheck Unit)))

(fn `I_GetAllPlayerUnits`
  (returns (Units :type "Array of Actor Object Reference"))
  (return (`/Game/GameplayFramework/Gamemode/BPC_TurnSystem.FriendlyUnits` (`self.BPC_TurnSystem`))))

(fn `I_GetEnemyUnits`
  (returns (Units :type "Array of Actor Object Reference"))
  (return (`/Game/GameplayFramework/Gamemode/BPC_TurnSystem.EnemyUnits` (`self.BPC_TurnSystem`))))

(fn `I_GetFriendlyUnits`
  (returns (Units :type "Array of Actor Object Reference"))
  (return (`/Game/GameplayFramework/Gamemode/BPC_TurnSystem.FriendlyUnits` (`self.BPC_TurnSystem`))))

(fn `I_GetMovementTiles`
  (params (Unit :type "Actor Object Reference"))
  (returns (Tiles :type "Array of IntPoint Structure"))
  (bind _unitdata (message `/Game/Units/Blueprints/Interface/I_Unit.I_GetData` Unit))
  (bind _index (message `/Game/Grid/Blueprints/Interface/I_Gridable.I_GetTileIndex` Unit))
  (bind _output_get (set `/Game/Grid/Blueprints/BP_Grid.TileInRange` (`/Game/Grid/Blueprints/Component/AC_BFS.GetTilesInRange` (`/Game/Grid/Blueprints/BP_Grid.AC_BFS` (`self.GridRef`)) _index (`/Game/Units/Blueprints/Datas/BP_UnitData.MovementRange` _unitdata) 50.0) (`self.GridRef`)))
  (return _output_get))

(fn `I_GetPath`
  (params (StartNode :type "IntPoint Structure") (EndNode :type "IntPoint Structure"))
  (returns (Path :type "Array of Vector Structure"))
  (return (`/Game/Grid/Blueprints/BP_Grid.GetTilesLocationByPath` (`self.GridRef`) StartNode EndNode 50.0)))

(fn `I_UnitIsAttacking`
  (returns (IsAttacking :type Boolean))
  (return (`self.IsAttacking`)))

(fn `MoveUnit`
  (params (UnitToMove :type "Actor Object Reference") (FirstTilePosition :type "IntPoint Structure") (LastTilePosition :type "IntPoint Structure"))
  (returns (OutCanMove :type Boolean))
  (locals (CanMove :type Boolean :default true))
  (bind _tilestomove (`/Game/Grid/Blueprints/BP_Grid.GetTilesLocationByPath` (`self.GridRef`) FirstTilePosition LastTilePosition 50.0))
  (bind _returnvalue (`KismetArrayLibrary.Array_Length` _tilestomove))
  (bind _canmove (message `/Game/Units/Blueprints/Interface/I_Unit.I_CanMove` UnitToMove))
  (if _canmove
    (if (> _returnvalue 0)
      ; If the tile where the unit wants to move is occupied, set "can move" to false
      (bind _index (`/Game/Grid/Blueprints/BP_Grid.GetTileIndexFromWorldLocation` (`self.GridRef`) (`|GetArrayItem` _tilestomove (- _returnvalue 1))))
      (bind _canmove_2 (`self.UnitCanMove` _index))
      (bind _output_get (set `local.CanMove` _canmove_2))
      (if _output_get
        (message `/Game/Units/Blueprints/Interface/I_Unit.I_Move` UnitToMove _tilestomove)
        (message `/Game/Grid/Blueprints/Tile/Interface/I_Tile.I_OnTileExit` (`/Game/Grid/Blueprints/BP_Grid.FindTile` (`self.GridRef`) (`local.FirstTilePosition`)))
        ; Da chiedere
        (`self.DisableInput` (`GameplayStatics.GetPlayerController` 0))
        (`/Game/Grid/Blueprints/BP_Grid.ResetOnlyTileInRange` (`self.GridRef`))
        (return (`local.CanMove`))
        (else
          (return _output_get)))
      (else
        (`KismetSystemLibrary.PrintString` "Path not found")))
    (else
      (`KismetSystemLibrary.PrintString` "Unit has already moved"))))

(fn `RemoveUnit`
  (params (Unit :type "Actor Object Reference"))
  (returns (Removed :type Boolean))
  (bind _bpc_turnsystem (`self.BPC_TurnSystem`))
  ; Is the unit to remove friendly?
  (if (`KismetArrayLibrary.Array_Contains` (`/Game/GameplayFramework/Gamemode/BPC_TurnSystem.FriendlyUnits` _bpc_turnsystem) Unit)
    ; If it is remove it
    (bind _returnvalue (`KismetArrayLibrary.Array_RemoveItem` (`/Game/GameplayFramework/Gamemode/BPC_TurnSystem.FriendlyUnits` (`self.BPC_TurnSystem`)) (`local.Unit`)))
    (return _returnvalue)
    (else
      ; Otherwise it's enemy, remove it as well
      (bind _returnvalue_2 (`KismetArrayLibrary.Array_RemoveItem` (`/Game/GameplayFramework/Gamemode/BPC_TurnSystem.EnemyUnits` _bpc_turnsystem) (`local.Unit`)))
      (return _returnvalue_2))))

(fn `SelectUnit`
  (params (TileRef :type "/Game/Grid/Blueprints/Tile/BP_Base_Tile Object Reference") (TileIndex :type "IntPoint Structure"))
  (returns (UnitFound :type Boolean))
  (locals (Found :type Boolean))
  (bind _unit (message `/Game/Grid/Blueprints/Tile/Interface/I_Tile.I_GetUnit` TileRef))
  (`/Engine/EditorBlueprintResources/StandardMacros.IsValid` _unit
    (:`Is Valid`
      (if (`KismetArrayLibrary.Array_Contains` (`/Game/GameplayFramework/Gamemode/BPC_TurnSystem.FriendlyUnits` (`self.BPC_TurnSystem`)) _unit)
        (bind _unitdata (message `/Game/Units/Blueprints/Interface/I_Unit.I_GetData` _unit))
        (bind _output_get (set `self.SelectedUnit` _unit))
        (bind _canmove (message `/Game/Units/Blueprints/Interface/I_Unit.I_CanMove` _output_get))
        (if _canmove
          (`/Game/Grid/Blueprints/BP_Grid.ShowMovementTiles` (`self.GridRef`) "NewEnumerator1" (`local.TileIndex`) (`/Game/Units/Blueprints/Datas/BP_UnitData.MovementRange` _unitdata) 50.0)
          (bind _output_get_2 (set `local.Found` true))
          (else
            (bind _canattack (message `/Game/Units/Blueprints/Interface/I_Unit.I_CanAttack` _output_get))
            (if _canattack
              (`/Game/Grid/Blueprints/BP_Grid.ShowAttackTiles` (`self.GridRef`) (`local.TileIndex`) (`/Game/Units/Blueprints/Datas/BP_UnitData.WeaponData` _unitdata))
              (set `self.IsAttacking` true)
              (bind _output_get_3 (set `local.Found` true))
              (return _output_get_3)
              (else
                (`KismetSystemLibrary.PrintString` "Unit doesn't have options left")
                (return (`local.Found`))))))
        (else
          (set `local.Found` false :!label _label))))
    (:`Is Not Valid`
      (goto _label)))
  (return _output_get_2))

(fn `UnitAttack`
  (params (AttackingUnit :type "Actor Object Reference") (TileToAttackIndex :type "IntPoint Structure"))
  (bind _returnvalue (`self.GetComponentByClass` AttackingUnit "/Game/GlobalBlueprints/Componets/AC_Combat.AC_Combat_C"))
  (bind _actor (`/Game/Grid/Blueprints/BP_Grid.FindTile` (`self.GridRef`) (`local.TileToAttackIndex`)))
  ; Checks if there is a unit on top of the tile
  (bind _unit (message `/Game/Grid/Blueprints/Tile/Interface/I_Tile.I_GetUnit` _actor))
  (`/Engine/EditorBlueprintResources/StandardMacros.IsValid` _unit
    (:`Is Valid`
      (message `/Game/Units/Blueprints/Interface/I_Unit.I_GetData` _unit)
      ; If it is in range attack
      (if (`KismetArrayLibrary.Array_Contains` (`/Game/Grid/Blueprints/BP_Grid.TileInRange` (`self.GridRef`)) (`local.TileToAttackIndex`))
        (`/Game/GlobalBlueprints/Componets/AC_Combat.Attack` _returnvalue _actor)
        (else
          ;[1 0 0 0.5] Uses the attack anyway (needs design choice)
          (`/Game/GlobalBlueprints/Componets/AC_Combat.Attack` _returnvalue null :!label _label))))
    (:`Is Not Valid`
      (goto _label)))
  ; Hides attack tiles and resets the state of the unit and grid
  (`/Game/Grid/Blueprints/BP_Grid.ResetOnlyTileInRange` (`self.GridRef`))
  (set `self.SelectedUnit` null)
  (message `/Game/GameplayFramework/Gamemode/Interfaces/BPI_GamemodeComunication.I_SwitchTo` self "NewEnumerator1")
  (set `self.IsAttacking` false))

(fn `UnitCanMove`
  (params (TargetTile :type "IntPoint Structure"))
  (returns (CanMove :type Boolean))
  (locals (NewLocalVar :type "Array of Boolean"))
  (bind (_actor _found) (`/Game/Grid/Blueprints/BP_Grid.FindTile` (`self.GridRef`) TargetTile))
  ; If the tile where the unit wants to move is occupied, set "can move" to false
  (if _found
    (bind _unit (message `/Game/Grid/Blueprints/Tile/Interface/I_Tile.I_GetUnit` _actor))
    (`/Engine/EditorBlueprintResources/StandardMacros.IsValid` _unit
      (:`Is Valid`
        (return false))
      (:`Is Not Valid`
        (return true)))
    (else
      (return false))))

(fn `UserConstructionScript`)