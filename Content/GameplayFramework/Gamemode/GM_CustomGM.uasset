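; Game mode for a grid tactics game that handles unit selection, movement, attacks and a reach-the-tile mission.
; Tile clicks select units, send them along BP_Grid paths or hit tiles, depending on attack state, through interface messages.
; Tick traces under the cursor to preview hovered units' movement range when none is selected.
; Reaching the random mission tile shows a point and picks another, until the threshold reveals a button.
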(event `self.ReceiveBeginPlay`
  (bind _returnvalue (`GameplayStatics.GetActorOfClass` "/Game/Grid/Blueprints/BP_Grid.BP_Grid_C"))
  (bind _output_get (set `self.GridRef` _returnvalue))
  (bind _output_get_2 (set `self.MissionTile` (`/Game/Grid/Blueprints/BP_Grid.GetRandomTileIndex` _output_get)))
  (`/Game/Grid/Blueprints/BP_Grid.ShowTileToReach` (`self.GridRef`) _output_get_2))

(event `/Game/GameplayFramework/Gamemode/Interfaces/BPI_GamemodeComunication.OnTileClick`
  (params (HitPosition :type "Vector Structure") (HitActor :type "Actor Object Reference"))
  (bind _gridref (`self.GridRef`))
  (bind _selectedunit (`self.SelectedUnit`))
  ; Tile pressed
  (bind _index (`/Game/Grid/Blueprints/BP_Grid.GetTileIndexFromWorldLocation` _gridref HitPosition))
  (bind (_value _returnvalue) (`BlueprintMapLibrary.Map_Find` (`/Game/Grid/Blueprints/BP_Grid.Tiles` _gridref) _index))
  (if _returnvalue
    (if (not (`self.IsAttacking`))
      ;; Questa parte serve per controllare quando muovere la pedina. Viene controllato se l'unità è già selezionata e non ho selezionato una nuova unità
      (bind _unitfound (`self.SelectUnit` _value _index))
      (if (and (not _unitfound) (`KismetSystemLibrary.IsValid` _selectedunit))
        (bind _index_2 (message `/Game/Grid/Blueprints/Interface/I_Gridable.I_GetIndex` _selectedunit))
        (`self.IsAttacking`
          (:`then`
            (`self.UnitAttack` (`self.SelectedUnit`) _index_2)
            (set `self.SelectedUnit` null))
          (:`else`
            (`self.MoveUnit` _selectedunit _index_2 _index)
            (set `self.SelectedUnit` null))))
      (elif (not (== (`self.GetUnitFromTileIndex` _index) _selectedunit))
        (`self.UnitAttack` _selectedunit _index)))))

(event `/Game/GameplayFramework/Gamemode/Interfaces/BPI_GamemodeComunication.OnTileReached`
  (params (TileIndex :type "IntPoint Structure"))
  (bind _maskthreshold (`self.MaskThreshold`))
  (bind _gridref (`self.GridRef`))
  ; Tile reached
  (if (<= (`self.MaskThreshold`) 3)
    (if (`KismetMathLibrary.Equal_IntPointIntPoint` TileIndex (`self.MissionTile`))
      (`/Game/UI/Mask/BP_FuctionLibrary.ShowPoint` _maskthreshold)
      (bind _result (`/Engine/EditorBlueprintResources/StandardMacros.IncrementInt` _maskthreshold)
        (:`  `
          (if (>= _result 3)
            (`/Game/UI/Mask/BP_FuctionLibrary.ShowButton`)
            (`/Game/Grid/Blueprints/BP_Grid.HideTileToReach` _gridref (`self.MissionTile`))
            (set `self.MissionTile` (make `IntPoint` -1 -1))
            (else
              (bind _output_get (set `self.MissionTile` (`/Game/Grid/Blueprints/BP_Grid.GetRandomTileIndex` (`self.GridRef`))))
              (`/Game/Grid/Blueprints/BP_Grid.ShowTileToReach` _gridref _output_get))))))))

(event `/Game/GameplayFramework/Gamemode/Interfaces/BPI_GamemodeComunication.SwitchTo`
  (params (State :type "/Game/Grid/Blueprints/Tile/Utilites/E_TileState Enum" :default "NewEnumerator0"))
  (bind _selectedunit (`self.SelectedUnit`))
  ; Switch to attack
  (`self.SelectedUnit`
    (:`then`
      (switch `/Game/Grid/Blueprints/Tile/Utilites/E_TileState` State
        (:`NewEnumerator1`
          (set `self.IsAttacking` false)
          (bind _index (message `/Game/Grid/Blueprints/Interface/I_Gridable.I_GetIndex` _selectedunit))
          (bind _unitdata (message `/Game/Units/Blueprints/Interface/I_Unit.I_GetUnitData` _selectedunit))
          (`/Game/Grid/Blueprints/BP_Grid.ShowTiles` (`self.GridRef`) "NewEnumerator1" _index (break `/Game/Units/Blueprints/Structure/S_UnitMovement` (`.Movement_5_691FD01246EAF1B61939889E36BAA629` (break `/Game/Units/Blueprints/Structure/S_UnitData` _unitdata)))))
        (:`NewEnumerator2`
          (set `self.IsAttacking` true)
          (bind _index_2 (message `/Game/Grid/Blueprints/Interface/I_Gridable.I_GetIndex` _selectedunit))
          (bind _unitdata_2 (message `/Game/Units/Blueprints/Interface/I_Unit.I_GetUnitData` _selectedunit))
          (`/Game/Grid/Blueprints/BP_Grid.ShowTiles` (`self.GridRef`) "NewEnumerator2" _index_2 (`.maxTiles_13_09C180494C504F9B4FA5E0ACB6FFE00C` (break `/Game/Units/Blueprints/Structure/S_UnitAttack` (break `/Game/Units/Blueprints/Structure/S_UnitData` _unitdata_2)))))))
    (:`else`)))

(event `self.ReceiveTick`
  (params (DeltaSeconds :type "Float (single-precision)"))
  (`self.CheckUnitHover`))

(fn `CheckUnitHover`
  (locals (UnderCursorUnit :type "Actor Object Reference") (PrevUnderCursorTile :type "/Game/Grid/Blueprints/Tile/BP_Base_Tile Object Reference"))
  (bind _location (`self.GetCursorLocationOnGrid` 0))
  (bind _index (`/Game/Grid/Blueprints/BP_Grid.GetTileIndexFromWorldLocation` (`self.GridRef`) _location))
  (set `local.PrevUnderCursorTile` (`self.UnderCursorTile`))
  (bind (_value _returnvalue) (`BlueprintMapLibrary.Map_Find` (`/Game/Grid/Blueprints/BP_Grid.Tiles` (`self.GridRef`)) _index))
  (set `self.UnderCursorTile` _value)
  (if _returnvalue
    (if (!= (`self.UnderCursorTile`) (`local.PrevUnderCursorTile`))
      (bind _unit (`/Game/Grid/Blueprints/Tile/BP_Base_Tile.I_GetUnit` (`self.UnderCursorTile`)))
      (bind _output_get (set `local.UnderCursorUnit` _unit))
      (`self.SelectedUnit`
        (:`then`)
        (:`else`
          (bind (_unitdata _hasget) (message `/Game/Units/Blueprints/Interface/I_Unit.I_GetUnitData` _output_get))
          (if _hasget
            (`/Game/Grid/Blueprints/BP_Grid.ShowTiles` (`self.GridRef`) "NewEnumerator5" (`/Game/Grid/Blueprints/Tile/BP_Base_Tile.Index` (`self.UnderCursorTile`)) (break `/Game/Units/Blueprints/Structure/S_UnitMovement` (`.Movement_5_691FD01246EAF1B61939889E36BAA629` (break `/Game/Units/Blueprints/Structure/S_UnitData` _unitdata))))
            (else
              (`/Game/Grid/Blueprints/BP_Grid.ResetOnlyTileInRange` (`self.GridRef`) :!label _label))))))
    (else
      (`local.PrevUnderCursorTile`
        (:`then`
          (`self.SelectedUnit`
            (:`then`)
            (:`else`
              (set `local.UnderCursorUnit` null)
              (goto _label))))
        (:`else`)))))

(fn `GetCursorLocationOnGrid`
  (params (PlayerIndex :type Integer))
  (returns (Location :type "Vector Structure"))
  (bind (_hitresult _returnvalue) (`PlayerController.GetHitResultUnderCursorByChannel` (`GameplayStatics.GetPlayerController` 0) "TraceTypeQuery4" false))
  (if _returnvalue
    (return (`.Location` (`GameplayStatics.BreakHitResult` _hitresult)))
    (else
      (return (-99999.0 -99999.0 -99999.0)))))

(fn `GetUnitFromTile`
  (params (TileRef :type "/Game/Grid/Blueprints/Tile/BP_Base_Tile Object Reference"))
  (returns (Unit :type "Actor Object Reference") (UnitFound :type Boolean))
  (bind _unit (message `/Game/Grid/Blueprints/Tile/Interface/I_Tile.I_GetUnit` TileRef))
  (return _unit (`KismetSystemLibrary.IsValid` _unit)))

(fn `GetUnitFromTileIndex`
  (params (TileIndex :type "IntPoint Structure"))
  (returns (Unit :type "Actor Object Reference") (UnitFound :type Boolean))
  (locals (Found :type Boolean))
  (bind (_value _returnvalue) (`BlueprintMapLibrary.Map_Find` (`/Game/Grid/Blueprints/BP_Grid.Tiles` (`self.GridRef`)) TileIndex))
  (bind _output_get (set `local.Found` _returnvalue))
  (if _output_get
    ; Setto e basta perché potrei arrivare anche dall'altra esecuzione
    (bind (_unit _unitfound) (`self.GetUnitFromTile` _value))
    (set `local.Found` _unitfound))
  (return _unit (`local.Found`)))

(fn `MoveUnit`
  (params (UnitToMove :type "Actor Object Reference") (FirstTilePosition :type "IntPoint Structure") (LastTilePosition :type "IntPoint Structure"))
  (bind _tilestomove (`/Game/Grid/Blueprints/BP_Grid.FindPath` (`self.GridRef`) FirstTilePosition LastTilePosition))
  (if (> (`KismetArrayLibrary.Array_Length` _tilestomove) 0)
    (message `/Game/Units/Blueprints/Interface/I_Unit.I_Move` UnitToMove _tilestomove)
    (message `/Game/Grid/Blueprints/Tile/Interface/I_Tile.I_OnTileExit` (`/Game/Grid/Blueprints/BP_Grid.FindTile` (`self.GridRef`) (`local.FirstTilePosition`)))
    ; Da chiedere
    (`self.DisableInput` (`GameplayStatics.GetPlayerController` 0))
    (`/Game/Grid/Blueprints/BP_Grid.ResetOnlyTileInRange` (`self.GridRef`))))

(fn `SelectUnit`
  (params (TileRef :type "/Game/Grid/Blueprints/Tile/BP_Base_Tile Object Reference") (TileIndex :type "IntPoint Structure"))
  (returns (UnitFound :type Boolean))
  (locals (Found :type Boolean))
  (bind _unit (message `/Game/Grid/Blueprints/Tile/Interface/I_Tile.I_GetUnit` TileRef))
  (`/Engine/EditorBlueprintResources/StandardMacros.IsValid` _unit
    (:`Is Valid`
      (set `local.Found` true)
      (bind _unitdata (message `/Game/Units/Blueprints/Interface/I_Unit.I_GetUnitData` _unit))
      (set `self.SelectedUnit` _unit)
      (`/Game/Grid/Blueprints/BP_Grid.ShowTiles` (`self.GridRef`) "NewEnumerator1" (`local.TileIndex`) (`.MaxTiles_2_4F3076CA471015173258E988AAF5F4F2` (break `/Game/Units/Blueprints/Structure/S_UnitMovement` (`.Movement_5_691FD01246EAF1B61939889E36BAA629` (break `/Game/Units/Blueprints/Structure/S_UnitData` _unitdata))))))
    (:`Is Not Valid`
      (set `local.Found` false)))
  (return (`local.Found`)))

(fn `UnitAttack`
  (params (Unit :type "Actor Object Reference") (TileToAttackIndex :type "IntPoint Structure"))
  (bind _actor (`/Game/Grid/Blueprints/BP_Grid.FindTile` (`self.GridRef`) (`local.TileToAttackIndex`)))
  (bind _unitdata (message `/Game/Units/Blueprints/Interface/I_Unit.I_GetUnitData` _actor))
  (message `/Game/GlobalBlueprints/Interface/I_Damageble.I_Hit` _actor Unit (break `/Game/Units/Blueprints/Structure/S_UnitAttack` (break `/Game/Units/Blueprints/Structure/S_UnitData` _unitdata))))

(fn `UserConstructionScript`)