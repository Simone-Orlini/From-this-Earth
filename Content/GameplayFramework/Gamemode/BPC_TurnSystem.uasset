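; Turn system component that alternates between the player and enemy teams and detects when either has no units left.
; EndCurrentTurn checks both unit arrays, then either broadcasts the winner or flips the turn, broadcasts the change and resets units through an interface message.
; Each StartEnemyAI call turns on the next enemy unit's AI controller by index, ending the turn once the list is exhausted.
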(event `EndCurrentTurn`
  (bind (_teamhasdied _playerwon) (`self.CheckTeamWon`))
  (if (not _teamhasdied)
    (bind _output_get (set `self.PlayerTurn` (not (`self.PlayerTurn`))))
    (`self.ChangeTurn` _output_get)
    (`self.ResetUnits`)
    (`self.PlayerTurn`
      (:`then`
        (set `self.currentEnemyIndex` 0))
      (:`else`))
    (else
      (`self.TeamWon` _playerwon))))

(event `StartEnemyAI`
  (if (< (`self.currentEnemyIndex`) (`KismetArrayLibrary.Array_Length` (`self.EnemyUnits`)))
    (bind _asaic_unit_test (cast `/Game/AI/TEST/AIC_UnitTEST` (`AIBlueprintHelperLibrary.GetAIController` (`|GetArrayItem` (`self.EnemyUnits`) (`self.currentEnemyIndex`)))))
    (`/Game/AI/TEST/AIC_UnitTEST.TurnOn` _asaic_unit_test)
    (`/Engine/EditorBlueprintResources/StandardMacros.IncrementInt` (`self.currentEnemyIndex`))
    (else
      (`self.EndCurrentTurn`))))

(fn `CheckTeamWon`
  (returns (TeamHasDied :type Boolean) (PlayerWon :type Boolean))
  (if (<= (`KismetArrayLibrary.Array_Length` (`self.FriendlyUnits`)) 0)
    (return true false)
    (elif (<= (`KismetArrayLibrary.Array_Length` (`self.EnemyUnits`)) 0)
      (return true true)
      (else
        (return false false)))))

(fn `ResetUnits`
  (`self.PlayerTurn`
    (:`then`
      (for _array_element (`self.FriendlyUnits`)
        (message `/Game/Units/Blueprints/Interface/I_Unit.I_Reset` _array_element)))
    (:`else`
      (for _array_element_2 (`self.EnemyUnits`)
        (message `/Game/Units/Blueprints/Interface/I_Unit.I_Reset` _array_element_2)))))