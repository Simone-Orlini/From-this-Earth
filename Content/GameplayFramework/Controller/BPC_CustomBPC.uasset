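; Player controller for tile-based mouse interaction that relays clicks and an attack toggle to the game mode.
; On BeginPlay it adds the IMC_CustomMC input mapping context and enables the cursor, click events and mouse-over events.
; A completed tile click traces under the cursor and, on a hit, sends the position and actor to the game mode.
; The attack input uses a FlipFlop to alternate the game mode between two enum states.
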(event `self.ReceiveBeginPlay`
  (`EnhancedInputSubsystemInterface.AddMappingContext` (pcsubsystem `EnhancedInputLocalPlayerSubsystem` self) "/Game/GameplayFramework/Controller/IMC_CustomMC.IMC_CustomMC" 1 (struct))
  (set `self.bShowMouseCursor` true)
  (set `self.bEnableClickEvents` true)
  (set `self.bEnableMouseOverEvents` true))

(event `EnhancedInput|/Game/GameplayFramework/Controller/IA_TileClick`
  (params (ActionValue :type Boolean) (ElapsedSeconds :type "Float (double-precision)") (TriggeredSeconds :type "Float (double-precision)") (InputAction :type "InputAction Object Reference" :default "/Game/GameplayFramework/Controller/IA_TileClick.IA_TileClick"))
  (:`Completed`
    (bind (_didhit _location _hittile) (`self.GetWorldMouseLocation`))
    (if _didhit
      (message `/Game/GameplayFramework/Gamemode/Interfaces/BPI_GamemodeComunication.OnTileClick` (`GameplayStatics.GetGameMode`) _location _hittile))))

(event `EnhancedInput|/Game/GameplayFramework/Controller/IA_AttackBtnPressed`
  (params (ActionValue :type Boolean) (ElapsedSeconds :type "Float (double-precision)") (TriggeredSeconds :type "Float (double-precision)") (InputAction :type "InputAction Object Reference" :default "/Game/GameplayFramework/Controller/IA_AttackBtnPressed.IA_AttackBtnPressed"))
  (bind _returnvalue (`GameplayStatics.GetGameMode`))
  (:`Completed`
    (`/Engine/EditorBlueprintResources/StandardMacros.FlipFlop`
      (:`A`
        (message `/Game/GameplayFramework/Gamemode/Interfaces/BPI_GamemodeComunication.SwitchTo` _returnvalue "NewEnumerator2"))
      (:`B`
        (message `/Game/GameplayFramework/Gamemode/Interfaces/BPI_GamemodeComunication.SwitchTo` _returnvalue "NewEnumerator1")))))

(fn `GetWorldMouseLocation`
  (returns (DidHit :type Boolean) (Location :type "Vector Structure") (HitTile :type "Actor Object Reference"))
  (bind (_hitresult _returnvalue) (`self.GetHitResultUnderCursorByChannel` self "TraceTypeQuery4" true))
  (bind (_bblockinghit _binitialoverlap _time _distance _location _impactpoint _normal _impactnormal _physmat _hitactor) (`GameplayStatics.BreakHitResult` _hitresult))
  (return _returnvalue _location _hitactor))

(fn `UserConstructionScript`)