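; Player controller for grid combat that handles mouse input for tile clicks, attack toggling and placing a mask actor.
; Enhanced Input actions trace under the cursor and message the game mode with the clicked tile or an attack-state switch.
; Right-click spawns the selected mask class at the grid-snapped cursor position, only once, inside BP_Grid bounds and if the first BP_Base_Unit found reports having a mask.
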(event `/Game/Mask/BPI_Mask_In_BPC_CombatBPC.selectMask`
  (params (ClassMask :type "Actor Class Reference"))
  (set `self.QualeMask?` ClassMask))

(event `Key|RightMouseButton`
  (params (Key :type "Key Structure"))
  (bind _returnvalue (`KismetMathLibrary.GridSnap_Float` (.x (`.Location` (`GameplayStatics.BreakHitResult` (`self.GetHitResultUnderCursorByChannel` "TraceTypeQuery1")))) 100.0))
  (bind _returnvalue_2 (`KismetMathLibrary.GridSnap_Float` (.y (`.Location` (`GameplayStatics.BreakHitResult` (`self.GetHitResultUnderCursorByChannel` "TraceTypeQuery1")))) 100.0))
  (:`Pressed`
    (bind _outactors (`GameplayStatics.GetAllActorsOfClass` "/Game/Units/Blueprints/BP_Base_Unit.BP_Base_Unit_C"))
    (bind _isequipped (message `/Game/Mask/Bp_Grab_Mask.GetHasMask` (`|GetArrayItem` _outactors)))
    (if _isequipped
      (bind _returnvalue_3 (`GameplayStatics.GetActorOfClass` "/Game/Grid/Blueprints/BP_Grid.BP_Grid_C"))
      (if (not (`self.IsPlace?`))
        (bind _returnvalue_4 (- _returnvalue (.x (`self.K2_GetActorLocation` _returnvalue_3))))
        (bind (_gridsize_x _gridsize_y) (break `IntVector2` (`/Game/Grid/Blueprints/BP_Grid.GridSize` _returnvalue_3)))
        (bind (_gridtilesize_x _gridtilesize_y) (`KismetMathLibrary.BreakVector` (`/Game/Grid/Blueprints/BP_Grid.GridTileSize` _returnvalue_3)))
        (bind _returnvalue_5 (/ (* _gridsize_x _gridtilesize_x) 2.0))
        (bind _returnvalue_6 (- _returnvalue_2 (.y (`self.K2_GetActorLocation` _returnvalue_3))))
        (bind _returnvalue_7 (/ (* _gridsize_y _gridtilesize_y) 2.0))
        (if (and (>= _returnvalue_4 (* _returnvalue_5 -1.0)) (<= _returnvalue_4 _returnvalue_5) (>= _returnvalue_6 (* _returnvalue_7 -1.0)) (<= _returnvalue_6 _returnvalue_7))
          (`KismetSystemLibrary.PrintString` (`KismetStringLibrary.Conv_BoolToString` _isequipped))
          (`|SpawnActorFromClass` (`self.QualeMask?`) (`KismetMathLibrary.MakeTransform` (`KismetMathLibrary.MakeVector` _returnvalue _returnvalue_2 (+ (.z (`.Location` (`GameplayStatics.BreakHitResult` (`self.GetHitResultUnderCursorByChannel` "TraceTypeQuery1")))) 30.0))) "Undefined" "MultiplyWithRoot" null null)
          (set `self.IsPlace?` true))))))

(event `self.ReceiveBeginPlay`
  (`EnhancedInputSubsystemInterface.AddMappingContext` (pcsubsystem `EnhancedInputLocalPlayerSubsystem` self) "/Game/GameplayFramework/Controller/IMC_CustomMC.IMC_CustomMC" 1 (struct))
  (set `self.bShowMouseCursor` true)
  (set `self.bEnableClickEvents` true)
  (set `self.bEnableMouseOverEvents` true))

(event `EnhancedInput|/Game/GameplayFramework/Controller/IA_TileClick`
  (params (ActionValue :type Boolean) (ElapsedSeconds :type "Float (double-precision)") (TriggeredSeconds :type "Float (double-precision)") (InputAction :type "InputAction Object Reference" :default "/Game/GameplayFramework/Controller/IA_TileClick.IA_TileClick"))
  (:`Completed`
    (bind (_didhit _location _hittile) (`self.GetWorldMouseLocation`))
    (if _didhit
      (message `/Game/GameplayFramework/Gamemode/Interfaces/BPI_GamemodeComunication.I_OnTileClick` (`GameplayStatics.GetGameMode`) _location _hittile))))

(event `EnhancedInput|/Game/GameplayFramework/Controller/IA_AttackBtnPressed`
  (params (ActionValue :type Boolean) (ElapsedSeconds :type "Float (double-precision)") (TriggeredSeconds :type "Float (double-precision)") (InputAction :type "InputAction Object Reference" :default "/Game/GameplayFramework/Controller/IA_AttackBtnPressed.IA_AttackBtnPressed"))
  (bind _returnvalue (`GameplayStatics.GetGameMode`))
  (:`Completed`
    (bind _isattacking (message `/Game/GameplayFramework/Gamemode/Interfaces/BPI_GamemodeComunication.I_UnitIsAttacking` (`GameplayStatics.GetGameMode`)))
    (if _isattacking
      (message `/Game/GameplayFramework/Gamemode/Interfaces/BPI_GamemodeComunication.I_SwitchTo` _returnvalue "NewEnumerator1")
      (else
        (message `/Game/GameplayFramework/Gamemode/Interfaces/BPI_GamemodeComunication.I_SwitchTo` _returnvalue "NewEnumerator2")))))

(fn `GetCombatController`
  (returns (Bpc_Combat :type "/Game/GameplayFramework/Controller/BPC_CombatBPC Object Reference"))
  (return self))

(fn `GetWorldMouseLocation`
  (returns (DidHit :type Boolean) (Location :type "Vector Structure") (HitTile :type "Actor Object Reference"))
  (bind (_hitresult _returnvalue) (`self.GetHitResultUnderCursorByChannel` self "TraceTypeQuery4" true))
  (bind (_bblockinghit _binitialoverlap _time _distance _location _impactpoint _normal _impactnormal _physmat _hitactor) (`GameplayStatics.BreakHitResult` _hitresult))
  (return _returnvalue _location _hitactor))

(fn `UserConstructionScript`)