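; AC_Combat is an actor component that gives its owner health, damage and an attack on other actors.
; Init sets the stats, and Attack sends an IHit interface message to the target's AC_Combat with owner and damage.
; A HasAttacked flag blocks repeat attacks and is not reset here.
; IHit subtracts health, calls OnHit, and at zero or below clamps health and calls OnDead.
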(event `/Game/GlobalBlueprints/Interface/I_Damageble.I_Hit`
  (params (fromWho :type "Actor Object Reference") (damage :type Integer))
  (set `self.CurrentHealth` (- (`self.CurrentHealth`) damage))
  (`self.OnHit` damage fromWho)
  (if (<= (`self.CurrentHealth`) 0)
    (set `self.CurrentHealth` 0)
    (`self.OnDead`)))

(fn `Attack`
  (params (Actor :type "Actor Object Reference"))
  (bind _returnvalue (`Actor.GetComponentByClass` Actor "AC_Combat_C"))
  (`self.HasAttacked`
    (:`then`
      (`KismetSystemLibrary.PrintString` "Unit has already attacked"))
    (:`else`
      (`/Engine/EditorBlueprintResources/StandardMacros.IsValid` _returnvalue
        (:`Is Valid`
          (message `/Game/GlobalBlueprints/Interface/I_Damageble.I_Hit` _returnvalue (`self.GetOwner`) (`self.Damage`))
          (set `self.HasAttacked` true))))))

(fn `Init`
  (params (MaxHealth :type Integer) (Damage :type Integer))
  (bind _output_get (set `self.MaxHealth` MaxHealth))
  (set `self.CurrentHealth` _output_get)
  (set `self.Damage` Damage))

(fn `IsDead`
  (returns (IsDead :type Boolean))
  (return (== (`self.CurrentHealth`) 0)))