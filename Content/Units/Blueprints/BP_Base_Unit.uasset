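; BP_Base_Unit is the base unit for grid-based combat, handling tile movement, per-unit action state and death.
; On BeginPlay it registers on the tile beneath it, initializes ACCombat from DataTable stats and subscribes to the game mode.
; Tick steps it along queued tile locations, then updates its tile, notifies the game mode and marks it moved.
; IReset clears move and attack flags; death unsubscribes, then destroys it after a short delay.
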(event `self.ReceiveBeginPlay`
  (bind _datatable (`self.DataTable`))
  (`KismetSystemLibrary.DelayUntilNextTick`)
  (`self.CheckTileUnder`)
  (`/Game/GlobalBlueprints/Componets/AC_Combat.Init` (`self.AC_Combat`) (`/Game/Units/Blueprints/Datas/BP_UnitData.MaxHealth` _datatable) (`/Game/Units/Blueprints/Datas/BP_UnitData.MovementRange` _datatable) (`/Game/Units/Blueprints/Datas/BP_UnitData.WeaponData_1` _datatable) (`/Game/Units/Blueprints/Datas/BP_UnitData.WeaponData_2` _datatable))
  (message `/Game/GameplayFramework/Gamemode/Interfaces/BPI_GamemodeComunication.I_SubscribeUnitToGameMode` (`GameplayStatics.GetGameMode`) self)
  (add `/Game/GlobalBlueprints/Componets/AC_Combat.OnDead` (`self.AC_Combat`) (`|CreateDelegate` :!event `OnDead_Event`)))

(event `self.ReceiveTick`
  (params (DeltaSeconds :type "Float (single-precision)"))
  (set `self.Delta second` DeltaSeconds)
  (if (`self.IsMoving`)
    (`self.Move`)))

(event `/Game/Units/Blueprints/Interface/I_Unit.I_Move`
  (params (TilesLocations :type "Array of Vector Structure (by ref)"))
  (`self.HasMoved`
    (:`then`)
    (:`else`
      (set `self.TilesToMove` TilesLocations)
      (set `self.IsMoving` true))))

(event `OnDead_Event`
  (message `/Game/GameplayFramework/Gamemode/Interfaces/BPI_GamemodeComunication.I_UnsubscribeUnitFromGameMode` (`GameplayStatics.GetGameMode`) self)
  ; Needed to show the unit die
  (`KismetSystemLibrary.Delay` 0.5)
  (`self.K2_DestroyActor`))

(event `/Game/Grid/Blueprints/Interface/I_Gridable.I_SetTileIndex`
  (params (intdex :type "IntPoint Structure"))
  (set `self.TileIndex` intdex))

(event `/Game/Units/Blueprints/Interface/I_Unit.I_Reset`
  (`self.ResetStats`))

(fn `CheckTileUnder`
  (bind _tiledata (message `/Game/GameplayFramework/Gamemode/Interfaces/BPI_GamemodeComunication.I_GetTileByWorldLoc` (`GameplayStatics.GetGameMode`) (`self.K2_GetActorLocation`)))
  (bind _output_get (set `self.TileIndex` (break `GridTileData` (break `TileData` _tiledata))))
  (bind _asgm_combat_gm (cast `/Game/GameplayFramework/Gamemode/GM_CombatGM` (`GameplayStatics.GetGameMode`)))
  (bind _tiledata_2 (`Tile.tileData` (`BlueprintMapLibrary.Map_Find` (`/Game/Grid/Blueprints/BP_Grid.Tiles` (`/Game/GameplayFramework/Gamemode/GM_CombatGM.GridRef` _asgm_combat_gm)) _output_get)))
  (bind (_gridtiledata _neighbors _biswalkable _actor _tilestatuses _outline _vfx _item) (break `TileData` _tiledata_2))
  (`|VariableSetRef` _tiledata_2 (make `TileData` _gridtiledata _neighbors _biswalkable self _tilestatuses _outline _vfx _item)))

(fn `I_CanAttack`
  (returns (CanAttack :type Boolean))
  (return (not (`/Game/GlobalBlueprints/Componets/AC_Combat.HasAttacked` (`self.AC_Combat`)))))

(fn `I_CanMove`
  (returns (CanMove :type Boolean))
  (return (not (`self.HasMoved`))))

(fn `I_GetData`
  (returns (UnitData :type "/Game/Units/Blueprints/Datas/BP_UnitData Object Reference"))
  (return (`self.DataTable`)))

(fn `I_GetTileIndex`
  (returns (index :type "IntPoint Structure"))
  (return (`self.TileIndex`)))

(fn `Move`
  (bind (_returnvalue_x _returnvalue_y _returnvalue_z) (`KismetMathLibrary.BreakVector` (`self.K2_GetActorLocation`)))
  (bind _tilestomove (`self.TilesToMove`))
  (bind _delta_second (`self.Delta second`))
  (bind (_output_x _output_y) (`KismetMathLibrary.BreakVector` (`|GetArrayItem` (`self.TilesToMove`))))
  (bind _maxwalkspeed (`CharacterMovementComponent.MaxWalkSpeed` (`self.CharacterMovement`)))
  (bind _returnvalue (- (`|GetArrayItem` (`self.TilesToMove`)) (`self.K2_GetActorLocation`)))
  (set `self.DistToNextTile` _returnvalue)
  (`self.K2_SetActorLocation` (+ (`self.K2_GetActorLocation`) (* (* (`KismetMathLibrary.Vector_Normal2D` _returnvalue) (`KismetMathLibrary.MakeVector` _maxwalkspeed _maxwalkspeed 1.0)) (`KismetMathLibrary.MakeVector` _delta_second _delta_second 1.0))))
  (if (<= (`KismetMathLibrary.VSizeXY` (`self.DistToNextTile`)) 6.0)
    (`self.K2_SetActorLocation` (`KismetMathLibrary.MakeVector` _output_x _output_y _returnvalue_z))
    (`KismetArrayLibrary.Array_Remove` _tilestomove)
    (if (<= (`KismetArrayLibrary.Array_Length` _tilestomove) 0)
      (set `self.IsMoving` false)
      (`self.CheckTileUnder`)
      (message `/Game/GameplayFramework/Gamemode/Interfaces/BPI_GamemodeComunication.I_OnTileReached` (`GameplayStatics.GetGameMode`) (`self.TileIndex`))
      (set `self.HasMoved` true))))

(fn `ResetStats`
  (set `self.HasMoved` false)
  (set `/Game/GlobalBlueprints/Componets/AC_Combat.HasAttacked` false (`self.AC_Combat`)))

(fn `UserConstructionScript`)