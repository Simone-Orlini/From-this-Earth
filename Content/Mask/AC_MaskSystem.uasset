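; Mask system component that places goal tiles on the combat grid and activates the mask the player picks as a reward for reaching one.
; SetTileToReach marks a random empty, unoccupied tile in movement range as ToReach, enables its VFX and blocks further placement.
; OnTileReach shows the mask selection HUD and re-allows placement.
; HUD clicks, bound a tick after BeginPlay, store the mask type and notify the combat game mode.
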(event `self.ReceiveBeginPlay`
  (`KismetSystemLibrary.DelayUntilNextTick`)
  (add `/Game/UI/Mask/BPW_UserWidget.OnMaskButtonClick` (`/Game/UI/Mask/BP_CombatHUD.MaskSelectionHUD` (`/Game/UI/Mask/BP_FuctionLibrary.Get HUD`)) (delegate `Event_OnMaskButtonClick`)))

(event `Event_OnMaskButtonClick`
  (params (MaskType :type "EMaskType Enum" :default "NONE"))
  (bind _output_get (set `self.Mask Type` MaskType))
  (`/Game/GameplayFramework/Gamemode/GM_CombatGM.OnMaskActive` (`self.Combat GM`) _output_get)
  (set `self.IsMaskActive` true))

(fn `OnTileReach`
  (`/Game/UI/Mask/BPW_UserWidget.Enable` (`/Game/UI/Mask/BP_CombatHUD.MaskSelectionHUD` (`/Game/UI/Mask/BP_FuctionLibrary.Get HUD`)))
  (set `self.CanSetNewTile` true))

(fn `SetTileToReach`
  (returns (Setted :type Boolean))
  (locals (TileEmpty :type "Array of GridTileData Structure") (CurrentIndex :type "IntPoint Structure") (TilesFound :type "Array of IntPoint Structure"))
  (bind _tileempty (`local.TileEmpty`))
  (bind _returnvalue (`KismetArrayLibrary.Array_Length` _tileempty))
  (bind _value (`BlueprintMapLibrary.Map_Find` (`/Game/Grid/Blueprints/BP_Grid.Tiles` (`/Game/GameplayFramework/Gamemode/GM_CombatGM.GridRef` (`self.Combat GM`))) (`local.CurrentIndex`)))
  (bind _output_index (break `GridTileData` (`|GetArrayItem` (`local.TileEmpty`) (`KismetMathLibrary.RandomIntegerInRange` 0 (- _returnvalue 1)))))
  (bind _gridtiledata (break `TileData` (`Tile.tileData` _value)))
  (bind (_index _transform) (break `GridTileData` _gridtiledata))
  (`self.CanSetNewTile`
    (:`then`
      (bind _output_get (set `local.TilesFound` (`/Game/GameplayFramework/Gamemode/GM_CombatGM.GetAllTileInMovementRange` (`self.Combat GM`))))
      (for _array_element _output_get
        (bind (_gridtiledata_2 _neighbors _biswalkable _actor) (break `TileData` (`Tile.tileData` (`BlueprintMapLibrary.Map_Find` (`/Game/Grid/Blueprints/BP_Grid.Tiles` (`/Game/GameplayFramework/Gamemode/GM_CombatGM.GridRef` (`self.Combat GM`))) _array_element))))
        (if (and (`|EnumEquality` (`.TileType` (break `GridTileData` _gridtiledata_2)) "Empty") (not (`KismetSystemLibrary.IsValid` _actor)))
          (`KismetArrayLibrary.Array_AddUnique` _tileempty _gridtiledata_2)))
      (if (> _returnvalue 0)
        (set `local.CurrentIndex` _output_index)
        (`|VariableSetRef` _gridtiledata (make `GridTileData` _index _transform "ToReach"))
        (`Tile.EnableVFX` _value)
        (set `self.CanSetNewTile` false)
        (return true)
        (else
          (return false))))
    (:`else`
      (return false))))