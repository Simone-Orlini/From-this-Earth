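; BP_TextureBaker is an editor utility actor in the Noise assets folder that bakes a material into a static texture asset.
; BakeTexture draws the assigned material into a render target, then saves that target as a Texture2D through an editor-only call.
; It prints a bake error if either input is missing; the event graph and construction script do nothing.
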(fn `BakeTexture`
  (if (and (`KismetSystemLibrary.IsValid` (`self.Render Target to Draw`)) (`KismetSystemLibrary.IsValid` (`self.Material to Draw From`)))
    (`KismetRenderingLibrary.DrawMaterialToRenderTarget` (`self.Render Target to Draw`) (`self.Material to Draw From`))
    (`KismetRenderingLibrary.RenderTargetCreateStaticTexture2DEditorOnly` (`self.Render Target to Draw`) "TextureFromRenderTarget")
    (else
      (`KismetSystemLibrary.PrintText` "Bake Error" true true (struct :`R` 1.0 :`G` 0.023611 :`B` 0.000196 :`A` 1.0)))))

(fn `UserConstructionScript`)