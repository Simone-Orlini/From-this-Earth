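; Base Blueprint for a tile-based unit that registers with the GameMode, can wear a mask on its head socket, and fights through a combat component.
; Move steps it along received tile locations each tick; on arrival, a downward trace updates its tile index and the GameMode is notified.
; DataTable stats initialize combat and the health bar; hits flash the mesh red, and death unsubscribes then destroys it after a delay.
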(event `/Game/Mask/Bp_Grab_Mask.prendiMask`
  (params (ActorMask :type "Actor Object Reference"))
  (set `self.HaveMask` true)
  (`self.K2_AttachToComponent` ActorMask (`self.Mesh`) "HeadSocket" "SnapToTarget" "KeepWorld" "KeepWorld" true))

(event `self.ReceiveBeginPlay`
  (bind _datatable (`self.DataTable`))
  (bind _maxhealth (`/Game/Units/Blueprints/Datas/BP_UnitData.MaxHealth` _datatable))
  (`KismetSystemLibrary.DelayUntilNextTick`)
  (`self.CheckTileUnder`)
  (`/Game/GlobalBlueprints/Componets/AC_Combat.Init` (`self.AC_Combat`) _maxhealth (`/Game/Weapons/BPDA_WeaponData.Damage` (`/Game/Units/Blueprints/Datas/BP_UnitData.WeaponData` _datatable)))
  (`/Game/Units/UI/BPWC_Healthar.SetHeath` (`self.BPWC_Healthar`) _maxhealth)
  (add `/Game/GlobalBlueprints/Componets/AC_Combat.OnHit` (`self.AC_Combat`) (`|CreateDelegate` :!event `Hit`))
  (message `/Game/GameplayFramework/Gamemode/Interfaces/BPI_GamemodeComunication.SubscribeUnitToGameMode` (`GameplayStatics.GetGameMode`) self)
  (add `/Game/GlobalBlueprints/Componets/AC_Combat.OnDead` (`self.AC_Combat`) (`|CreateDelegate` :!event `OnDead_Event`)))

(event `self.ReceiveTick`
  (params (DeltaSeconds :type "Float (single-precision)"))
  (set `self.Delta second` DeltaSeconds)
  (if (`self.IsMoving`)
    (`self.Move`)))

(event `self.I_Move`
  (params (TilesLocations :type "Array of Vector Structure (by ref)"))
  (set `self.TilesToMove` TilesLocations)
  (set `self.IsMoving` true))

(event `Hit`
  (params (damage :type Integer) (FromWho :type "Actor Object Reference"))
  (`/Game/Units/UI/BPWC_Healthar.UpdateHealth` (`self.BPWC_Healthar`) damage)
  (`KismetSystemLibrary.K2_SetTimerDelegate` (delegate `ChangeMaterial`) 0.1)
  (`PrimitiveComponent.SetMaterial` (`self.Mesh`) 0 "/Game/Materials/MI_Red.MI_Red"))

(event `ChangeMaterial`
  (`PrimitiveComponent.SetMaterial` (`self.Mesh`) 0 null))

(event `OnDead_Event`
  (message `/Game/GameplayFramework/Gamemode/Interfaces/BPI_GamemodeComunication.UnsubscribeUnitFromGameMode` (`GameplayStatics.GetGameMode`) self)
  ; Needed to show the unit die
  (`KismetSystemLibrary.Delay` 0.5)
  (`self.K2_DestroyActor`))

(event `self.I_SetIndex`
  (params (intdex :type "IntPoint Structure"))
  (set `self.TileIndex` intdex))

(fn `CheckTileUnder`
  (bind _returnvalue (`self.K2_GetActorLocation`))
  (bind _outhit (`KismetSystemLibrary.LineTraceSingle` :`Start` _returnvalue :`End` (- _returnvalue (0.0 0.0 500.0)) :`TraceChannel` "TraceTypeQuery4" :`DrawDebugType` "ForDuration"))
  (bind (_bblockinghit _binitialoverlap _time _distance _location _impactpoint _normal _impactnormal _physmat _hitactor) (`GameplayStatics.BreakHitResult` _outhit))
  (message `/Game/Grid/Blueprints/Tile/Interface/I_Tile.I_OnTileEnter` _hitactor self)
  (bind _index (message `/Game/Grid/Blueprints/Interface/I_Gridable.I_GetTileIndex` _hitactor))
  (set `self.TileIndex` _index))

(fn `GetHasMask`
  (returns (isEquipped :type Boolean))
  (return (`self.HaveMask`)))

(fn `I_CanAttack`
  (returns (CanAttack :type Boolean))
  (return false))

(fn `I_CanMove`
  (returns (CanMove :type Boolean))
  (return false))

(fn `I_GetData`
  (returns (UnitData :type "/Game/Units/Blueprints/Datas/BP_UnitData Object Reference"))
  (return (`self.DataTable`)))

(fn `I_GetTileIndex`
  (returns (index :type "IntPoint Structure"))
  (return (`self.TileIndex`)))

(fn `Move`
  (bind (_returnvalue_x _returnvalue_y _returnvalue_z) (`KismetMathLibrary.BreakVector` (`self.K2_GetActorLocation`)))
  (bind _tilestomove (`self.TilesToMove`))
  (bind _delta_second (`self.Delta second`))
  (bind (_output_x _output_y) (`KismetMathLibrary.BreakVector` (`|GetArrayItem` (`self.TilesToMove`))))
  (bind _maxwalkspeed (`CharacterMovementComponent.MaxWalkSpeed` (`self.CharacterMovement`)))
  (bind _returnvalue (- (`|GetArrayItem` (`self.TilesToMove`)) (`self.K2_GetActorLocation`)))
  (set `self.DistToNextTile` _returnvalue)
  (`self.K2_SetActorLocation` (+ (`self.K2_GetActorLocation`) (* (* (`KismetMathLibrary.Vector_Normal2D` _returnvalue) (`KismetMathLibrary.MakeVector` _maxwalkspeed _maxwalkspeed 1.0)) (`KismetMathLibrary.MakeVector` _delta_second _delta_second 1.0))))
  (if (<= (`KismetMathLibrary.VSizeXY` (`self.DistToNextTile`)) 6.0)
    (`self.K2_SetActorLocation` (`KismetMathLibrary.MakeVector` _output_x _output_y _returnvalue_z))
    (`KismetArrayLibrary.Array_Remove` _tilestomove)
    (if (<= (`KismetArrayLibrary.Array_Length` _tilestomove) 0)
      (set `self.IsMoving` false)
      (`self.CheckTileUnder`)
      (message `/Game/GameplayFramework/Gamemode/Interfaces/BPI_GamemodeComunication.OnTileReached` (`GameplayStatics.GetGameMode`) (`self.TileIndex`)))))

(fn `UserConstructionScript`)