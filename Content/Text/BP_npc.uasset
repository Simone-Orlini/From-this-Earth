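; NPC Blueprint that shows dialogue when an actor tagged Player begins overlapping its Box trigger.
; The first overlap creates a WBP_Dialogue widget, seeds its row name from DialogueID, adds it to the viewport and shows a line from Dialogue_DataTable.
; While that widget reference is valid, later overlaps advance the first top-level dialogue widget found, then show the next line on the stored one.
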(event `self.Box.OnComponentBeginOverlap`
  (params (OverlappedComponent :type "PrimitiveComponent Object Reference") (OtherActor :type "Actor Object Reference") (OtherComp :type "PrimitiveComponent Object Reference") (OtherBodyIndex :type Integer) (bFromSweep :type Boolean) (SweepResult :type "HitResult Structure (by ref)"))
  (bind _wbp_dialogue (`self.WBP_Dialogue`))
  (if (`self.ActorHasTag` OtherActor "Player")
    (`/Engine/EditorBlueprintResources/StandardMacros.IsValid` (`self.WBP_Dialogue`)
      (:`Is Valid`
        (bind _foundwidgets (`WidgetBlueprintLibrary.GetAllWidgetsOfClass` "/Game/Text/WBP_Dialogue.WBP_Dialogue_C"))
        (bind _output (`|GetArrayItem` _foundwidgets))
        (`/Engine/EditorBlueprintResources/StandardMacros.IsValid` _output
          (:`Is Valid`
            (`/Game/Text/WBP_Dialogue.AdvanceDialogue` _output))))
      (:`Is Not Valid`
        (bind _returnvalue (`|CreateWidget` "/Game/Text/WBP_Dialogue.WBP_Dialogue_C"))
        (set `self.WBP_Dialogue` _returnvalue)
        (set `/Game/Text/WBP_Dialogue.CurrebtRowName` (`self.DialogueID`) _wbp_dialogue)
        (`UserWidget.AddToViewport` _wbp_dialogue 0)))
    (`/Game/Text/WBP_Dialogue.ShowNextLine` _wbp_dialogue "/Game/Text/Dialogue_DataTable.Dialogue_DataTable")))

(fn `UserConstructionScript`)