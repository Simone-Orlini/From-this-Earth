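; Test dialogue component that opens and advances an on-screen WBP_Dialogue widget when an interaction event fires.
; The first interaction creates the widget, seeds its row name from DialogueID and shows a line from Dialogue_DataTable.
; Later interactions advance the first top-level WBP_Dialogue found by class search rather than the stored reference.
; Fine_Interaction only hides the widget, leaving the reference set.
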(event `Dialogue_Iteraction`
  (bind _wbp_dialogue (`self.WBP_Dialogue`))
  (`/Engine/EditorBlueprintResources/StandardMacros.IsValid` (`self.WBP_Dialogue`)
    (:`Is Valid`
      (bind _foundwidgets (`WidgetBlueprintLibrary.GetAllWidgetsOfClass` "/Game/Text/WBP_Dialogue.WBP_Dialogue_C"))
      (bind _output (`|GetArrayItem` _foundwidgets))
      (`/Engine/EditorBlueprintResources/StandardMacros.IsValid` _output
        (:`Is Valid`
          (`/Game/Text/WBP_Dialogue.AdvanceDialogue` _output))))
    (:`Is Not Valid`
      (bind _returnvalue (`|CreateWidget` "/Game/Text/WBP_Dialogue.WBP_Dialogue_C"))
      (set `self.WBP_Dialogue` _returnvalue)
      (set `/Game/Text/WBP_Dialogue.CurrebtRowName` (`self.DialogueID`) _wbp_dialogue)
      (`UserWidget.AddToViewport` _wbp_dialogue 0)
      (`/Game/Text/WBP_Dialogue.ShowNextLine` _wbp_dialogue "/Game/Text/Dialogue_DataTable.Dialogue_DataTable"))))

(event `Fine_Interaction`
  (`Widget.SetVisibility` (`self.WBP_Dialogue`) "Hidden"))